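; Interactable box container that holds items and shows its contents in an inventory widget when used.
; On authority, the construction script assigns the sphere as collision and fills the inventory with the configured amount of each item class in ConstructItems.
; The overlap-and-use action calls the parent, then creates an Inventory widget for player character 0, passes it the stored items and adds it to the viewport.
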(fn `ActionOnOverlapAndUse`
  (`parent.ActionOnOverlapAndUse`)
  (bind _returnvalue (`|GenericCreateObject` "/Game/Shipping/Blueprints/HUD/Inventories/Inventory.Inventory_C" (`GameplayStatics.GetPlayerCharacter` 0)))
  (`/Game/Shipping/Blueprints/HUD/Inventories/Inventory.GetItems` _returnvalue (`/Game/Shipping/Blueprints/Environment/Interactable/Containers/Base/BP_Inventory.Items` (`self.BP_Inventory`)))
  (`UserWidget.AddToViewport` _returnvalue 0))

(fn `UserConstructionScript`
  (`parent.UserConstructionScript`)
  (`/Engine/EditorBlueprintResources/ActorMacros.Switch Has Authority`
    (:`Authority`
      (set `self.Collision` (`self.Sphere`))
      (for _array_element (`self.ConstructItems`)
        (bind (_item _amount) (break `/Game/Shipping/Blueprints/Environment/Interactable/Containers/Base/ConstructItem` _array_element))
        (for _ (range (+ _amount 1))
          (bind _returnvalue (`|GenericCreateObject` _item self))
          (`/Game/Shipping/Blueprints/Environment/Interactable/Containers/Base/BP_Inventory.AddItem` (`self.BP_Inventory`) _returnvalue))))))