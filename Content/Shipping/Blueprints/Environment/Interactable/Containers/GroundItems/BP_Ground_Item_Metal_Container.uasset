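; Ground item for a metal container that a player picks up by overlapping and using it.
; It overrides ActionOnOverlapAndUse to run the parent logic, cast the overlapping actor to Player and call GetItem with InvID 0 on that player's BP_Inventory component.
; The actor destroys itself only when GetItem succeeds.
; All other behavior comes from the parent class, as the event graph holds only disabled stubs.
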(fn `ActionOnOverlapAndUse`
  (`parent.ActionOnOverlapAndUse`)
  (bind _asplayer (cast `/Game/Shipping/Blueprints/Entities/Player` (`self.OverlappingActor`)))
  (bind _success (`/Game/Shipping/Blueprints/Environment/Interactable/Containers/Base/BP_Inventory.GetItem` (`self.BP_Inventory`) (`self.GetComponentByClass` _asplayer "/Game/Shipping/Blueprints/Environment/Interactable/Containers/Base/BP_Inventory.BP_Inventory_C") 0))
  (if _success
    (`self.K2_DestroyActor`)))

(fn `UserConstructionScript`
  (`parent.UserConstructionScript`))