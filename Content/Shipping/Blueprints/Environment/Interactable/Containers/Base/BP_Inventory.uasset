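; BP_Inventory is a capacity-limited item container in the interactable containers Blueprints, storing Items up to Size.
; AddItem appends while space remains, returning whether the item count is still below Size afterwards.
; GetItem passes an indexed item to another inventory's AddItem and, on a true result, blanks the source slot without shrinking the array.
; GetItems and CanAddMore expose contents and free space.
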(fn `AddItem`
  (params (Item :type "/Game/Shipping/Blueprints/Environment/Interactable/Items/Base/BP_Item Object Reference (by ref)"))
  (returns (Successful :type Boolean))
  (bind _returnvalue (< (`KismetArrayLibrary.Array_Length` (`self.Items`)) (`KismetMathLibrary.Conv_Int64ToInt` (`self.Size`))))
  (if _returnvalue
    (`KismetArrayLibrary.Array_Add` (`self.Items`) Item))
  (return _returnvalue))

(fn `CanAddMore`
  (returns (CanAddMore :type Boolean))
  (return (< (`KismetMathLibrary.Conv_IntToInt64` (`KismetArrayLibrary.Array_Length` (`self.Items`))) (`self.Size`))))

(fn `Get Items`
  (returns (Items :type "Array of /Game/Shipping/Blueprints/Environment/Interactable/Items/Base/BP_Item Object Reference"))
  (return (`self.Items`)))

(fn `GetItem`
  (params (Inventory :type "/Game/Shipping/Blueprints/Environment/Interactable/Containers/Base/BP_Inventory Object Reference (by ref)") (InvID :type Integer64))
  (returns (Success :type Boolean))
  (bind _returnvalue (`KismetMathLibrary.Conv_Int64ToInt` InvID))
  (bind _successful (`self.AddItem` Inventory (`|GetArrayItem` (`self.Items`) _returnvalue)))
  (if _successful
    (`KismetArrayLibrary.Array_Set` (`self.Items`) _returnvalue))
  (return _successful))