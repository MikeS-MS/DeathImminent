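; Base ground item container that holds an item in its inventory and transfers it when a player overlaps and uses it.
; On the authority, the construction script constructs the configured item class and adds it to the inventory unless creation is skipped.
; The authority also assigns the sphere as the collision component.
; The server use action runs the parent logic, then moves the item at index 0 to the target.
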(event `self.ReceiveBeginPlay`
  (`parent.ReceiveBeginPlay`)
  (`/Engine/EditorBlueprintResources/ActorMacros.Switch Has Authority`
    (:`Authority`
      (set `self.CollisionComponent` (`self.Sphere`)))))

(fn `Server_ActionOnOverlapAndUse`
  (params (Player :type "/Game/Shipping/Blueprints/Entities/Player Object Reference (by ref)"))
  (`parent.Server_ActionOnOverlapAndUse` Player)
  (`self.MoveItemToTarget` 0))

(fn `UserConstructionScript`
  (`parent.UserConstructionScript`)
  (`/Engine/EditorBlueprintResources/ActorMacros.Switch Has Authority`
    (:`Authority`
      (set `self.Collision` (`self.Sphere`))
      (if (not (`self.SkipCreatingItem`))
        (bind _returnvalue (`|GenericCreateObject` (`self.ItemToConstruct`) self))
        (`/Game/Shipping/Blueprints/Environment/Interactable/Containers/Base/BP_Inventory.AddItem` (`self.BP_Inventory`) _returnvalue)))))