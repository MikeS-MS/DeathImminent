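; Door widget mesh component that spins while visible and shows one of two materials based on its Phase state.
; Tick updates roll, pitch and yaw through UpdateRotation, using per-axis settings for enable, step and direction.
; The rotation mixes per-frame steps with a delta-time term, so speed depends on frame rate.
; OnRep_Phase calls SwitchMaterial to swap between start and secondary materials, tracking the current one.
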(event `self.ReceiveBeginPlay`
  (bind _startmaterial (`self.StartMaterial`))
  (`self.SetMaterial` 0 _startmaterial)
  (set `self.CurrentMaterial` _startmaterial))

(event `self.ReceiveTick`
  (params (DeltaSeconds :type "Float (single-precision)"))
  (if (not (`self.bHiddenInGame`))
    (bind _finalrotation (`self.UpdateRotation` DeltaSeconds (.roll (`self.RelativeRotation`)) (`self.Roll`)))
    (bind _finalrotation_2 (`self.UpdateRotation` DeltaSeconds (.pitch (`self.RelativeRotation`)) (`self.Pitch`)))
    (bind _finalrotation_3 (`self.UpdateRotation` DeltaSeconds (.yaw (`self.RelativeRotation`)) (`self.Yaw`)))
    (`self.K2_SetRelativeRotation` (`KismetMathLibrary.MakeRotator` _finalrotation _finalrotation_2 _finalrotation_3))))

(fn `OnRep_Phase`
  (`self.Switch Material`))

(fn `Switch Material`
  (bind _secondarymaterial (`self.SecondaryMaterial`))
  (bind _startmaterial (`self.StartMaterial`))
  (if (`self.Phase`)
    (`self.SetMaterial` 0 _secondarymaterial)
    (set `self.CurrentMaterial` _secondarymaterial)
    (else
      (`self.SetMaterial` 0 _startmaterial)
      (set `self.CurrentMaterial` _startmaterial))))

(fn `UpdateRotation`
  (params (DeltaTime :type "Float (double-precision) (by ref)") (Component :type "Float (double-precision) (by ref)") (RotationInfo :type "ComponentRotate Structure (by ref)"))
  (returns (FinalRotation :type "Float (double-precision)"))
  (bind (_benablemoving _movedirection _moveby) (break `ComponentRotate` RotationInfo))
  (bind _returnvalue (`KismetMathLibrary.Conv_BoolToDouble` _benablemoving))
  (bind _returnvalue_2 (* _moveby _returnvalue))
  (return (+ (+ (+ Component _returnvalue_2) (* (* DeltaTime _returnvalue_2) (`KismetMathLibrary.Conv_IntToDouble` _movedirection))) (* _returnvalue (`self.UpdateBy`)))))