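; Interactable sliding door that moves its mesh between closed and open world positions according to the Open flag.
; At BeginPlay the authority derives the end position from per-axis move settings and mesh bounds.
; On tick, the authority steps replicated CurrentPosition at constant speed, and its OnRep moves the mesh.
; RemoteTick runs the same interpolation directly on the mesh, and both paths flag FinishedAnimation at either endpoint.
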(event `self.ReceiveBeginPlay`
  (bind _mesh (`self.Mesh`))
  (`parent.ReceiveBeginPlay`)
  (`/Engine/EditorBlueprintResources/ActorMacros.Switch Has Authority`
    (:`Authority`
      (bind _output_get (set `self.BeginPosition` (`SceneComponent.K2_GetComponentLocation` _mesh)))
      (bind _returnvalue (`SlidingDoor.SetUpPositions` (`self.X`) (`self.Y`) (`self.Z`) (`.BoxExtent` (`KismetSystemLibrary.GetComponentBounds` _mesh)) _output_get))
      (set `self.EndPosition` _returnvalue))))

(event `OpenDoorClient`
  (`self.UpdateDoorClient`))

(event `Update Door`
  (`/Engine/EditorBlueprintResources/ActorMacros.Switch Has Authority`
    (:`Authority`
      (`self.UpdateDoorServer`))))

(fn `CheckIfReachedTargetClient`
  (params (DeltaTime :type "Float (double-precision)") (Target :type "Vector Structure"))
  (bind _returnvalue (`SceneComponent.K2_GetComponentLocation` (`self.Mesh`)))
  (if (!= _returnvalue Target)
    (bind _position (`self.GetFinalPosition` _returnvalue Target DeltaTime))
    (`SceneComponent.K2_SetWorldLocation` (`self.Mesh`) _position false false))
  (return))

(fn `CheckIfReachedTargetServer`
  (params (DeltaTime :type "Float (double-precision)") (Target :type "Vector Structure"))
  (bind _returnvalue (`SceneComponent.K2_GetComponentLocation` (`self.Mesh`)))
  (if (!= _returnvalue Target)
    (bind _position (`self.GetFinalPosition` _returnvalue Target DeltaTime))
    (set `self.CurrentPosition` _position))
  (return))

(fn `GetFinalPosition`
  (params (CurrentPosition :type "Vector Structure (by ref)") (TargetPosition :type "Vector Structure (by ref)") (DeltaTime :type "Float (double-precision) (by ref)"))
  (returns (Position :type "Vector Structure"))
  (bind _updateby (`self.UpdateBy`))
  (return (`KismetMathLibrary.MakeVector` (`KismetMathLibrary.FInterpTo_Constant` (.x CurrentPosition) (.x TargetPosition) DeltaTime _updateby) (`KismetMathLibrary.FInterpTo_Constant` (.y CurrentPosition) (.y TargetPosition) DeltaTime _updateby) (`KismetMathLibrary.FInterpTo_Constant` (.z CurrentPosition) (.z TargetPosition) DeltaTime _updateby))))

(fn `OnRep_CurrentPosition`
  (`SceneComponent.K2_SetWorldLocation` (`self.Mesh`) (`self.CurrentPosition`) false false)
  (return))

(fn `OnTick`
  (`parent.OnTick`)
  (`self.Update Door`))

(fn `RemoteTick`
  (`parent.RemoteTick`)
  (`self.OpenDoorClient`))

(fn `SetComponent`
  (params (Axis :type "Float (double-precision)") (Size :type "Float (double-precision)") (MovePos :type "MovePosition Structure (by ref)"))
  (returns (OutAxis :type "Float (double-precision)"))
  (locals (TempAxis :type Boolean))
  (bind (_benablemoving _movedirection _benableadditive _additivemovevalue _bcustommovevalue _moveby) (break `MovePosition` MovePos))
  (return (+ Axis (* (+ (+ (* (* (`KismetMathLibrary.Conv_BoolToDouble` _benablemoving) Size) (`KismetMathLibrary.Conv_BoolToDouble` (not _bcustommovevalue))) (* (`KismetMathLibrary.Conv_BoolToDouble` _benableadditive) _additivemovevalue)) (* (`KismetMathLibrary.Conv_BoolToDouble` _bcustommovevalue) _moveby)) (`KismetMathLibrary.Conv_IntToDouble` _movedirection)))))

(fn `UpdateDoorClient`
  (bind _returnvalue (`GameplayStatics.GetWorldDeltaSeconds`))
  (bind _returnvalue_2 (`SceneComponent.K2_GetComponentLocation` (`self.Mesh`)))
  (if (`self.Open`)
    (`self.CheckIfReachedTargetClient` _returnvalue (`self.EndPosition`))
    (else
      (`self.CheckIfReachedTargetClient` _returnvalue (`self.BeginPosition`))))
  (if (or (== _returnvalue_2 (`self.BeginPosition`)) (== _returnvalue_2 (`self.EndPosition`)))
    (set `self.FinishedAnimation` true)))

(fn `UpdateDoorServer`
  (bind _returnvalue (`GameplayStatics.GetWorldDeltaSeconds`))
  (bind _returnvalue_2 (`SceneComponent.K2_GetComponentLocation` (`self.Mesh`)))
  (if (`self.Open`)
    (`self.CheckIfReachedTargetServer` _returnvalue (`self.EndPosition`))
    (else
      (`self.CheckIfReachedTargetServer` _returnvalue (`self.BeginPosition`))))
  (if (or (== _returnvalue_2 (`self.BeginPosition`)) (== _returnvalue_2 (`self.EndPosition`)))
    (set `self.FinishedAnimation` true)))

(fn `UserConstructionScript`
  (`parent.UserConstructionScript`))