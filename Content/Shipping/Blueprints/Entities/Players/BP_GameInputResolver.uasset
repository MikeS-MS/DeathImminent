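; BP_GameInputResolver translates gameplay input events into actions on the player.
; Press and release events for jump, run and use each check that the Player reference is valid before forwarding.
; Jump starts and stops jumping, run switches between running and walking through Server-prefixed calls, and use press triggers Interact.
; Use release performs no action, and BeginPlay and Tick are unused.
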(event `self.OnJumpPress`
  (bind _player (`self.Player`))
  (`/Engine/EditorBlueprintResources/StandardMacros.IsValid` _player
    (:`Is Valid`
      (`Character.Jump` _player))))

(event `self.OnJumpRelease`
  (bind _player (`self.Player`))
  (`/Engine/EditorBlueprintResources/StandardMacros.IsValid` _player
    (:`Is Valid`
      (`Character.StopJumping` _player))))

(event `self.OnRunPress`
  (bind _player (`self.Player`))
  (`/Engine/EditorBlueprintResources/StandardMacros.IsValid` _player
    (:`Is Valid`
      (`/Game/Shipping/Blueprints/Entities/Players/BP_Player.Server_SetRunning` _player))))

(event `self.OnRunRelease`
  (bind _player (`self.Player`))
  (`/Engine/EditorBlueprintResources/StandardMacros.IsValid` _player
    (:`Is Valid`
      (`/Game/Shipping/Blueprints/Entities/Players/BP_Player.Server_SetWalking` _player))))

(event `self.OnUsePress`
  (bind _player (`self.Player`))
  (`/Engine/EditorBlueprintResources/StandardMacros.IsValid` _player
    (:`Is Valid`
      (`/Game/Shipping/Blueprints/Entities/Players/BP_Player.Interact` _player))))

(event `self.OnUseRelease`
  (`/Engine/EditorBlueprintResources/StandardMacros.IsValid` (`self.Player`)))