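; Usable door Blueprint that extends a parent interactable: a server-authoritative use toggles it open or closed unless it is locked or mid-animation.
; Setup finds door and frame meshes by component tag and passes a rotation speed to its DoorWidget components.
; Overlap shows or hides two outer rings.
; Widget ticks switch the widgets' phase to reflect the locked state, comparing current materials to decide when a change is needed.
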(event `Toggle Door`
  (`self.Toggle`))

(event `SetHidden`
  (`SceneComponent.SetHiddenInGame` (`self.Outer_Ring`) true true)
  (`SceneComponent.SetHiddenInGame` (`self.Outer_Ring1`) true true))

(event `SetNotHidden`
  (`SceneComponent.SetHiddenInGame` (`self.Outer_Ring`) false true)
  (`SceneComponent.SetHiddenInGame` (`self.Outer_Ring1`) false true))

(fn `ActionOnEndOverlap`
  (`parent.ActionOnEndOverlap`)
  (`self.SetHidden`)
  (set `self.Hidden` true))

(fn `ActionOnOverlap`
  (`parent.ActionOnOverlap`)
  (`self.SetNotHidden`)
  (set `self.Hidden` false))

(fn `ActionOnOverlapAndUse`
  (`parent.ActionOnOverlapAndUse`)
  (`/Engine/EditorBlueprintResources/ActorMacros.Switch Has Authority`
    (:`Authority`
      (if (`self.CanUseAgain`)
        (`self.Toggle Door`)))))

(fn `ChangeColor`
  (bind _returnvalue (`self.K2_GetComponentsByClass` "/Game/Shipping/Blueprints/DoorWidget.DoorWidget_C"))
  (bind _returnvalue_2 (`self.K2_GetComponentsByClass` "/Game/Shipping/Blueprints/DoorWidget.DoorWidget_C"))
  (if (`self.Locked`)
    (if (`self.CanBeChanged`)
      (for _array_element _returnvalue
        (set `/Game/Shipping/Blueprints/DoorWidget.Phase` true _array_element))
      (set `self.CanBeChanged` false)
      (else
        (for _array_element_2 _returnvalue
          (if (not (== (`/Game/Shipping/Blueprints/DoorWidget.CurrentMaterial` _array_element_2) (`/Game/Shipping/Blueprints/DoorWidget.SecondaryMaterial` _array_element_2)))
            (set `self.CanBeChanged` true)
            (break)))))
    (elif (`self.CanBeChanged`)
      (for _array_element_3 _returnvalue_2
        (set `/Game/Shipping/Blueprints/DoorWidget.Phase` false _array_element_3))
      (set `self.CanBeChanged` false)
      (else
        (for _array_element_4 _returnvalue_2
          (if (not (== (`/Game/Shipping/Blueprints/DoorWidget.CurrentMaterial` _array_element_4) (`/Game/Shipping/Blueprints/DoorWidget.StartMaterial` _array_element_4)))
            (set `self.CanBeChanged` true)
            (break)))))))

(fn `InitialSetup`
  (`parent.InitialSetup`)
  (for _array_element (`self.GetComponentsByTag` "/Script/Engine.StaticMeshComponent" "Door")
    (set `self.Mesh` _array_element)
    (for _array_element_2 (`self.GetComponentsByTag` "/Script/Engine.StaticMeshComponent" "DoorFrame")
      (set `self.FrameMesh` _array_element_2))
    (for _array_element_3 (`self.K2_GetComponentsByClass` "/Game/Shipping/Blueprints/DoorWidget.DoorWidget_C")
      (set `/Game/Shipping/Blueprints/DoorWidget.UpdateBy` (`self.RotateWidgetSpeed`) _array_element_3))))

(fn `Toggle`
  (if (`self.Locked`)
    _
    (elif (`self.FinishedAnimation`)
      (set `self.Open` (not (`self.Open`)))
      (set `self.FinishedAnimation` false)
      (set `self.CanUseAgain` false))))

(fn `UserConstructionScript`
  (`parent.UserConstructionScript`))

(fn `WidgetSetup`
  (`parent.WidgetSetup`))

(fn `WidgetTick`
  (`parent.WidgetTick`)
  (`self.ChangeColor`))

(fn `WidgetTickServer`
  (`parent.WidgetTickServer`)
  (`self.ChangeColor`))