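; Base Blueprint for interactable objects that a Player can use while inside a trigger Box.
; The server tracks the overlapping Player and, each tick, calls the use hook while IsUsing is set, otherwise re-arms CanUseAgain.
; Empty functions serve as override points for setup, overlap, use and tick, with tick hooks split between authority and remote.
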(event `self.ReceiveBeginPlay`
  (`/Engine/EditorBlueprintResources/ActorMacros.Switch Has Authority`
    (:`Authority`
      (`self.WidgetSetup`)
      (`self.InitialSetup`))))

(event `self.ReceiveTick`
  (params (DeltaSeconds :type "Float (single-precision)"))
  (`/Engine/EditorBlueprintResources/ActorMacros.Switch Has Authority`
    (:`Authority`
      (bind _asplayer (cast `/Game/Shipping/Blueprints/Player` (`self.OverlappingActor`))
        (:`then`
          (if (`/Game/Shipping/Blueprints/Player.isUsing` _asplayer)
            (`self.OnOverlapAndUse`)
            (else
              (set `self.CanUseAgain` true :!label _label))))
        (:`CastFailed`
          (goto _label)))
      (`self.OnTick`)
      (`self.WidgetTickServer`))
    (:`Remote`
      (`self.RemoteTick`)
      (`self.WidgetTick`))))

(event `self.Box.OnComponentBeginOverlap`
  (params (OverlappedComponent :type "PrimitiveComponent Object Reference") (OtherActor :type "Actor Object Reference") (OtherComp :type "PrimitiveComponent Object Reference") (OtherBodyIndex :type Integer) (bFromSweep :type Boolean) (SweepResult :type "HitResult Structure (by ref)"))
  (`/Engine/EditorBlueprintResources/ActorMacros.Switch Has Authority`
    (:`Authority`
      (bind _asplayer (cast `/Game/Shipping/Blueprints/Player` OtherActor))
      (set `self.ActorInside` true)
      (set `self.OverlappingActor` _asplayer)
      (`self.ActionOnOverlap`))))

(event `self.Box.OnComponentEndOverlap`
  (params (OverlappedComponent :type "PrimitiveComponent Object Reference") (OtherActor :type "Actor Object Reference") (OtherComp :type "PrimitiveComponent Object Reference") (OtherBodyIndex :type Integer))
  (`/Engine/EditorBlueprintResources/ActorMacros.Switch Has Authority`
    (:`Authority`
      (set `self.ActorInside` false)
      (set `self.OverlappingActor` null)
      (`self.ActionOnEndOverlap`))))

(event `OnOverlapAndUse`
  (`self.ActionOnOverlapAndUse`))

(fn `ActionOnEndOverlap`)

(fn `ActionOnOverlap`)

(fn `ActionOnOverlapAndUse`)

(fn `InitialSetup`)

(fn `OnTick`)

(fn `RemoteTick`)

(fn `UserConstructionScript`)

(fn `WidgetSetup`)

(fn `WidgetTick`)

(fn `WidgetTickServer`)