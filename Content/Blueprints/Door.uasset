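; Door actor Blueprint whose open state flips when the inherited overlap action fires.
; InitialSetup extends the parent's by caching the StaticMeshComponent tagged "Door" as Mesh.
; ActionOnOverlap calls the parent, then ToggleDoor, which runs Toggle to invert Open only if FinishedAnimation is true, then clears that flag.
; The file contains no logic that moves the mesh or sets FinishedAnimation back to true.
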(event `Toggle Door`
  (`self.Toggle`))

(fn `ActionOnOverlap`
  (`parent.ActionOnOverlap`)
  (`self.Toggle Door`))

(fn `InitialSetup`
  (`parent.InitialSetup`)
  (for _array_element (`self.GetComponentsByTag` "/Script/Engine.StaticMeshComponent" "Door")
    (set `self.Mesh` _array_element)))

(fn `Toggle`
  (if (`self.FinishedAnimation`)
    (set `self.Open` (not (`self.Open`)))
    (set `self.FinishedAnimation` false)))

(fn `UserConstructionScript`
  (`parent.UserConstructionScript`))