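; BP_TestWeapon is a test weapon that assembles a modular gun from hardcoded Dev parts on BeginPlay.
; It looks up each part through WeaponManager and adds a static mesh component using that part's first in-game model.
; The grip sits at the origin, and the engine's SupportedParts offsets position the engine, barrel, gas chamber, magazine and stock.
; Barrel and gas chamber share the same offset.
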(event `self.ReceiveBeginPlay`
  (bind _returnvalue (subsystem `WeaponManager`))
  (bind _returnvalue_ingamemodels (break `WeaponPartStats` (`WeaponManager.GetStatsForPart` _returnvalue (make `WeaponPartName` "Stock" "DevStock"))))
  (bind _returnvalue_ingamemodels_2 (break `WeaponPartStats` (`WeaponManager.GetStatsForPart` _returnvalue (make `WeaponPartName` "PrimaryGrip" "DevPrimaryGrip"))))
  (bind _returnvalue_ingamemodels_3 (break `WeaponPartStats` (`WeaponManager.GetStatsForPart` _returnvalue (make `WeaponPartName` "GasChamber" "DevGasChamber"))))
  (bind _returnvalue_ingamemodels_4 (break `WeaponPartStats` (`WeaponManager.GetStatsForPart` _returnvalue (make `WeaponPartName` "Barrel" "DevBarrel"))))
  (bind _returnvalue_ingamemodels_5 (break `WeaponPartStats` (`WeaponManager.GetStatsForPart` _returnvalue (make `WeaponPartName` "Magazine" "DevMagazine"))))
  (bind (_returnvalue_ingamemodels_6 _returnvalue_supportedparts) (break `WeaponPartStats` (`WeaponManager.GetStatsForPart` _returnvalue (make `WeaponPartName` "Engine" "DevEngine"))))
  (bind (_output_slot _output_type _output_offset) (break `WeaponPartType` (`|GetArrayItem` _returnvalue_supportedparts 2)))
  (bind (_output_slot_2 _output_type_2 _output_offset_2) (break `WeaponPartType` (`|GetArrayItem` _returnvalue_supportedparts 1)))
  (bind (_output_slot_3 _output_type_3 _output_offset_3) (break `WeaponPartType` (`|GetArrayItem` _returnvalue_supportedparts)))
  (bind (_output_slot_4 _output_type_4 _output_offset_4) (break `WeaponPartType` (`|GetArrayItem` _returnvalue_supportedparts 3)))
  (bind _returnvalue_2 (* _output_offset_3 -1.0))
  (bind _returnvalue_3 (+ _returnvalue_2 _output_offset))
  (bind _returnvalue_4 (`AddComponent|NODE_AddStaticMeshComponent-1`))
  (`StaticMeshComponent.SetStaticMesh` _returnvalue_4 (`|GetArrayItem` _returnvalue_ingamemodels_2))
  (bind _returnvalue_5 (`AddComponent|NODE_AddStaticMeshComponent-0` :`RelativeTransform` (`KismetMathLibrary.MakeTransform` _returnvalue_2)))
  (`StaticMeshComponent.SetStaticMesh` _returnvalue_5 (`|GetArrayItem` _returnvalue_ingamemodels_6))
  (bind _returnvalue_6 (`AddComponent|NODE_AddStaticMeshComponent-2` :`RelativeTransform` (`KismetMathLibrary.MakeTransform` _returnvalue_3)))
  (`StaticMeshComponent.SetStaticMesh` _returnvalue_6 (`|GetArrayItem` _returnvalue_ingamemodels_4))
  (bind _returnvalue_7 (`AddComponent|NODE_AddStaticMeshComponent-3` :`RelativeTransform` (`KismetMathLibrary.MakeTransform` _returnvalue_3)))
  (`StaticMeshComponent.SetStaticMesh` _returnvalue_7 (`|GetArrayItem` _returnvalue_ingamemodels_3))
  (bind _returnvalue_8 (`AddComponent|NODE_AddStaticMeshComponent-6` :`RelativeTransform` (`KismetMathLibrary.MakeTransform` (+ _returnvalue_2 _output_offset_2))))
  (`StaticMeshComponent.SetStaticMesh` _returnvalue_8 (`|GetArrayItem` _returnvalue_ingamemodels_5))
  (bind _returnvalue_9 (`AddComponent|NODE_AddStaticMeshComponent-8` :`RelativeTransform` (`KismetMathLibrary.MakeTransform` (+ _returnvalue_2 _output_offset_4))))
  (`StaticMeshComponent.SetStaticMesh` _returnvalue_9 (`|GetArrayItem` _returnvalue_ingamemodels)))

(fn `UserConstructionScript`)