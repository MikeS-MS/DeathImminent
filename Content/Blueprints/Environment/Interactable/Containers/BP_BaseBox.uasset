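; Base box container actor that acts as both a movable object and an inventory holder in the environment.
; On BeginPlay, the authority passes the Model to its BPBaseMovable and BPBaseInventory components.
; Two separate collision volumes forward begin and end overlaps to their matching component, PickupCollision to movable and InventoryCollision to inventory, leaving the interaction logic to those components.
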(event `self.ReceiveBeginPlay`
  (bind _model (`self.Model`))
  (`/Engine/EditorBlueprintResources/ActorMacros.Switch Has Authority`
    (:`Authority`
      (`|ExecutionSequence`
        (:`then_0`
          (`/Game/Blueprints/Environment/Interactable/BP_BaseInteractable.SetComponent` (`self.BP_BaseMovable`) _model))
        (:`then_1`
          (`/Game/Blueprints/Environment/Interactable/BP_BaseInteractable.SetComponent` (`self.BP_BaseInventory`) _model))))))

(event `self.Pickup Collision.OnComponentBeginOverlap`
  (params (OverlappedComponent :type "PrimitiveComponent Object Reference") (OtherActor :type "Actor Object Reference") (OtherComp :type "PrimitiveComponent Object Reference") (OtherBodyIndex :type Integer) (bFromSweep :type Boolean) (SweepResult :type "HitResult Structure (by ref)"))
  (`/Game/Blueprints/Environment/Interactable/BP_BaseInteractable.Event_OnCollisionBeginOverlap` (`self.BP_BaseMovable`) OverlappedComponent OtherActor OtherComp OtherBodyIndex bFromSweep SweepResult))

(event `self.Pickup Collision.OnComponentEndOverlap`
  (params (OverlappedComponent :type "PrimitiveComponent Object Reference") (OtherActor :type "Actor Object Reference") (OtherComp :type "PrimitiveComponent Object Reference") (OtherBodyIndex :type Integer))
  (`/Game/Blueprints/Environment/Interactable/BP_BaseInteractable.Event_OnCollisionEndOverlap` (`self.BP_BaseMovable`) OverlappedComponent OtherActor OtherComp OtherBodyIndex))

(event `self.Inventory Collision.OnComponentBeginOverlap`
  (params (OverlappedComponent :type "PrimitiveComponent Object Reference") (OtherActor :type "Actor Object Reference") (OtherComp :type "PrimitiveComponent Object Reference") (OtherBodyIndex :type Integer) (bFromSweep :type Boolean) (SweepResult :type "HitResult Structure (by ref)"))
  (`/Game/Blueprints/Environment/Interactable/BP_BaseInteractable.Event_OnCollisionBeginOverlap` (`self.BP_BaseInventory`) OverlappedComponent OtherActor OtherComp OtherBodyIndex bFromSweep SweepResult))

(event `self.Inventory Collision.OnComponentEndOverlap`
  (params (OverlappedComponent :type "PrimitiveComponent Object Reference") (OtherActor :type "Actor Object Reference") (OtherComp :type "PrimitiveComponent Object Reference") (OtherBodyIndex :type Integer))
  (`/Game/Blueprints/Environment/Interactable/BP_BaseInteractable.Event_OnCollisionEndOverlap` (`self.BP_BaseInventory`) OverlappedComponent OtherActor OtherComp OtherBodyIndex))

(fn `UserConstructionScript`)