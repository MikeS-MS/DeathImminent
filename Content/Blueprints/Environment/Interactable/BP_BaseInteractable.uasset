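; Base interactable that tracks when a BP_Player enters or leaves its collision and provides hooks for using it.
; Overlap handlers split into server events on authority and local events for the locally controlled player.
; The server sets itself as the player's Interactable on enter and clears it on leave if still current.
; Local hooks and post-enter are empty, server use returns true by default, and SetComponent stores ComponentToHit.
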(event `Event_OnCollisionBeginOverlap`
  (params (`Overlapped Component` :type "ActorComponent Object Reference") (`Other Actor` :type "Actor Object Reference") (`Other Comp` :type "ActorComponent Object Reference") (`Other Body Index` :type Integer) (`From Sweep` :type Boolean) (`Sweep Result` :type "HitResult Structure"))
  (bind _asbp_player (cast `/Game/Blueprints/Entities/Players/BP_Player` `Other Actor`))
  (`|ExecutionSequence`
    (:`then_0`
      (if (`Actor.HasAuthority` (`self.GetOwner`))
        (`self.Server_OnPlayerEnter` _asbp_player)))
    (:`then_1`
      (if (`Pawn.IsLocallyControlled` _asbp_player)
        (`self.Local_OnPlayerEnter` _asbp_player)))))

(event `Event_OnCollisionEndOverlap`
  (params (`Overlapped Component` :type "ActorComponent Object Reference") (`Other Actor` :type "Actor Object Reference") (`Other Comp` :type "ActorComponent Object Reference") (`Other Body Index` :type Integer))
  (bind _asbp_player (cast `/Game/Blueprints/Entities/Players/BP_Player` `Other Actor`))
  (`|ExecutionSequence`
    (:`then_0`
      (if (`Actor.HasAuthority` (`self.GetOwner`))
        (`self.Server_OnPlayerLeave` _asbp_player)))
    (:`then_1`
      (if (`Pawn.IsLocallyControlled` _asbp_player)
        (`self.Local_OnPlayerLeave` _asbp_player)))))

(event `Local_OnPlayerEnter`
  (params (Player :type "/Game/Blueprints/Entities/Players/BP_Player Object Reference")))

(event `Local_OnPlayerLeave`
  (params (Player :type "/Game/Blueprints/Entities/Players/BP_Player Object Reference")))

(event `Local_OnPlayerUseSuccess`
  (params (Player :type "/Game/Blueprints/Entities/Players/BP_Player Object Reference")))

(event `Local_OnPlayerUseFailed`
  (params (Player :type "/Game/Blueprints/Entities/Players/BP_Player Object Reference")))

(event `Server_OnPlayerEnter`
  (params (Player :type "/Game/Blueprints/Entities/Players/BP_Player Object Reference"))
  (set `/Game/Blueprints/Entities/Players/BP_Player.Interactable` self Player)
  (`self.Server_OnPostPlayerEnter` Player))

(event `Server_OnPostPlayerEnter`
  (params (Player :type "/Game/Blueprints/Entities/Players/BP_Player Object Reference")))

(event `Server_OnPlayerLeave`
  (params (Player :type "/Game/Blueprints/Entities/Players/BP_Player Object Reference (by ref)"))
  (if (== (`/Game/Blueprints/Entities/Players/BP_Player.Interactable` Player) self)
    (set `/Game/Blueprints/Entities/Players/BP_Player.Interactable` null Player)))

(event `SetComponent`
  (params (NewComponent :type "ActorComponent Object Reference"))
  (set `self.ComponentToHit` NewComponent))

(fn `Server_OnPlayerUse`
  (params (Player :type "/Game/Blueprints/Entities/Players/BP_Player Object Reference"))
  (returns (Success :type Boolean))
  (return true))