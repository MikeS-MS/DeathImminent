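; BP_Grid is a block-based building grid that divides a bounded volume, centered on the world origin, into chunk actors.
; On BeginPlay it sets the bounds, spawns and attaches a square XY layout of chunks, half-fills them and updates their meshes.
; TryHitBlock and TryPlaceBlock bounds-check a world location, convert it to a flattened chunk index and forward the call to that chunk.
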(event EventBeginPlay
  (Setup|Setup))

(fn ConstructionScript)

(fn IsLocationInsideGrid
  (params (Location :type Vector))
  (return (Class|KismetMathLibrary|IsPointinBoxBox Location (Variables|Stats|GetMapBounds))))

(fn GetSize
  (params (AsUnits :type Boolean))
  (bind _cellsize (Variables|Stats|GetCellSize))
  (bind _heightinunits (Variables|Stats|GetHeightInUnits))
  (bind _widthinunits (Variables|Stats|GetWidthInUnits))
  (if AsUnits
    (return (Utilities|Struct|MakeIntPoint _widthinunits _heightinunits))
    (else
      (return (Utilities|Struct|MakeIntPoint (/ _widthinunits _cellsize) (/ _heightinunits _cellsize))))))

(fn GetChunkSizeinUnits
  (return (|({DD1C2743-44FF-9A18-DF94-2FA5CA324F7E}*{3C21F4F0-458A-34B2-322C-A787302D1258}))))

(fn ConvertLocationtoArrayUsable
  (params (Location :type Vector))
  (return (|(Vec((X+({4A62CA90-424D-8156-0C71-7A8314BB4DF6}/2)),(Y+({4A62CA90-424D-8156-0C71-7A8314BB4DF6}/2)),(Z+({CC216E14-4D1B-C3CC-38C5-0781B4151B4A}/2)))) (.x Location) (.y Location) (.z Location))))

(fn ConverttoChunkIndexVector
  (params (Location :type Vector))
  (return (Class|KismetMathLibrary|FTruncVector (|(Vec(((Floor(X))/ChunkSize),((Floor(Y))/ChunkSize),((Floor(Z))/ChunkSize))) (.x Location) (.y Location) (.z Location) (Utilities|GetChunkSizeinUnits)))))

(fn TryHitBlock
  (params (Location :type Vector))
  (bind _result (Utilities|ConvertLocationtoArrayUsable Location))
  (bind _chunks (Variables|Data|GetChunks))
  (bind _result_2 (Utilities|ConverttoChunkIndexVector _result))
  (bind _index (Utilities|ConverttoArrayIndex _result_2))
  (if (Utilities|IsLocationInsideGrid Location)
    (if (Utilities|Array|IsValidIndex _chunks _index)
      (Class|Chunk|TryHitBlock (Utilities|Array|Get(acopy) _chunks _index) Location))))

(fn TryPlaceBlock
  (params (Location :type Vector))
  (bind _result (Utilities|ConvertLocationtoArrayUsable Location))
  (bind _chunks (Variables|Data|GetChunks))
  (bind _result_2 (Utilities|ConverttoChunkIndexVector _result))
  (bind _index (Utilities|ConverttoArrayIndex _result_2))
  (if (Utilities|IsLocationInsideGrid Location)
    (if (Utilities|Array|IsValidIndex _chunks _index)
      (Class|Chunk|TryPlaceBlock (Utilities|Array|Get(acopy) _chunks _index) Location))))

(fn Setup
  (if (not (Variables|Stats|GetIsSetup))
    (Setup|SetBounds)
    (Setup|SpawnChunks)
    (Test|FillAllChunks)
    (Variables|Stats|SetIsSetup true)))

(fn SpawnChunks
  (LocalVariables|SetChunkSizeInUnits (Utilities|GetChunkSizeinUnits))
  (LocalVariables|SetChunkAmount (|({4A62CA90-424D-8156-0C71-7A8314BB4DF6}/{36E089BA-4718-F70F-D85A-08992143BFA4})))
  (LocalVariables|SetStartXY (|(({4A62CA90-424D-8156-0C71-7A8314BB4DF6}/2)*NegOne) -1))
  (for _index (range 0 (- (LocalVariables|GetChunkAmount) 1))
    (for _index_2 (range 0 (- (LocalVariables|GetChunkAmount) 1))
      (bind _returnvalue (Game|SpawnActorfromClass "/Script/DeathImminent.Chunk" (Math|Transform|MakeTransform (|(Vec((X+({36E089BA-4718-F70F-D85A-08992143BFA4}/2)),(Y+({36E089BA-4718-F70F-D85A-08992143BFA4}/2)),Z)) (|({C6D3295C-48D4-F761-A623-1E948FEEA98D}+(IndexX*{36E089BA-4718-F70F-D85A-08992143BFA4})) _index) (|({C6D3295C-48D4-F761-A623-1E948FEEA98D}+(IndexY*{36E089BA-4718-F70F-D85A-08992143BFA4})) _index_2)) "0, 0, 0" "1.000000,1.000000,1.000000") "Undefined" 0 0))
      (Transformation|AttachActorToActor _returnvalue self "None" "KeepWorld" "KeepWorld" "KeepWorld" false)
      (bind _output_get (LocalVariables|SetCurrentChunk _returnvalue))
      (Class|Chunk|SetInformation _output_get (Variables|Stats|GetChunkSizeInBlocks) (|({CC216E14-4D1B-C3CC-38C5-0781B4151B4A}/{3C21F4F0-458A-34B2-322C-A787302D1258})) (Variables|Stats|GetCellSize))
      (Class|Chunk|FillChunkZeroed _output_get)
      (Utilities|Array|SetArrayElem (Variables|Data|GetChunks) (Utilities|ConverttoArrayIndex (Utilities|Struct|MakeIntVector _index _index_2 0)) (LocalVariables|GetCurrentChunk) true))))

(fn OnRepChunks)

(fn SetBounds
  (bind _returnvalue (|(Vec(({4A62CA90-424D-8156-0C71-7A8314BB4DF6}/2),({4A62CA90-424D-8156-0C71-7A8314BB4DF6}/2),({CC216E14-4D1B-C3CC-38C5-0781B4151B4A}/2)))))
  (Variables|Stats|SetMapBounds (Math|Box|MakeBox (* _returnvalue -1) _returnvalue)))

(fn FillAllChunks
  (for _array_element (Variables|Data|GetChunks)
    (Class|Chunk|FillChunkHalf _array_element)
    (Class|Chunk|UpdateMeshes _array_element)))

(fn ConverttoArrayIndex
  (params (IndexVector :type Int%20Vector%20Structure))
  (return (|(X+(Y*Width)) (.x IndexVector) (.y IndexVector) (|(({4A62CA90-424D-8156-0C71-7A8314BB4DF6}/{3C21F4F0-458A-34B2-322C-A787302D1258})/{DD1C2743-44FF-9A18-DF94-2FA5CA324F7E})))))