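; BP_BaseItem is a base item Blueprint for stackable, weighted items, with stub defaults for consumability (false) and description (empty).
; AddAmount fills the stack up to MaxAmount and returns any overflow, while SetAmount clamps its input between one and MaxAmount.
; GetWeight scales unit weight by the current amount, IsFull checks the cap, and GetID looks up the item's class through BPItemManager.
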(fn `AddAmount`
  (params (Amount :type Integer))
  (returns (AmountLeft :type Integer))
  (locals (Temp :type Integer))
  (bind _maxamount (`self.MaxAmount`))
  (bind _returnvalue (+ Amount (`self.CurrentAmount`)))
  (bind _output_get (set `local.Temp` _returnvalue))
  (if (> _returnvalue (`self.MaxAmount`))
    (set `self.CurrentAmount` _maxamount)
    (return (- _output_get _maxamount))
    (else
      (set `self.CurrentAmount` _returnvalue)
      (return 0))))

(fn `CanBeConsumed`
  (returns (CanBeConsumed :type Boolean))
  (return false))

(fn `GetDescription`
  (returns (Description :type String))
  (return ""))

(fn `GetID`
  (returns (ID :type "/Game/Blueprints/Entities/Inventory/S_ItemID Structure"))
  (bind _id (`/Game/Blueprints/Subsystems/BP_ItemManager.GetID` (subsystem `/Game/Blueprints/Subsystems/BP_ItemManager`) (`GameplayStatics.GetObjectClass` self)))
  (return _id))

(fn `GetWeight`
  (returns (Weight :type "Float (double-precision)"))
  (return (* (`self.CurrentAmount`) (`self.Weight`))))

(fn `IsFull`
  (returns (Full :type Boolean))
  (return (== (`self.CurrentAmount`) (`self.MaxAmount`))))

(fn `SetAmount`
  (params (Amount :type Integer))
  (`|VariableSetRef` 0 (`KismetMathLibrary.Clamp` Amount 1 (`self.MaxAmount`))))