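; DoorTrigger is a trigger Blueprint that lets the player toggle a door while the trigger is occupied.
; Begin and end overlap events set an Inside flag, without checking which actor overlaps.
; While Inside is true, Tick polls the first-person character's IsUsing flag and calls Toggle on the Door component of a referenced Actor.
; Toggle repeats every frame that IsUsing stays true, as this graph does not reset it.
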(event `self.ReceiveBeginPlay`
  ;[1 1 1] Set default values for flags
  (set `self.Inside` false))

(event `self.ReceiveActorBeginOverlap`
  (params (OtherActor :type "Actor Object Reference"))
  ;[1 1 1] Set player/actor is Inside the box flag
  (set `self.Inside` true))

(event `self.ReceiveActorEndOverlap`
  (params (OtherActor :type "Actor Object Reference"))
  ;[1 1 1] Set player/actor is Inside the box flag
  (set `self.Inside` false))

(event `self.ReceiveTick`
  (params (DeltaSeconds :type "Float (single-precision)"))
  ;[1 1 1] Update Door State (Open/Close)
  (if (`self.Inside`)
    (bind _asfirst_person_character (cast `/Game/Blueprints/FirstPersonCharacter` (`GameplayStatics.GetPlayerCharacter` 0)))
    (if (`/Game/Blueprints/FirstPersonCharacter.isUsing` _asfirst_person_character)
      (`Door.Toggle` (`self.GetComponentByClass` (`self.Actor`) "/Script/HorrorEscape.Door")))))

(fn `UserConstructionScript`)