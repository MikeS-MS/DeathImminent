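; BP_BaseItem is a base item Blueprint holding a stack amount, weight, item type and rarity.
; Amount functions cap the stack at MaxAmount, with AddAmount returning the overflow, and queries report fullness and total stack weight.
; Rarity getters read name, ordering, shader and widget from the rarity class defaults, while the ID comes from BPItemManager.
; Description, custom-data serialization and Consume are empty stubs.
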(event EventBeginPlay)

(event EventTick
  (params (DeltaSeconds :type Float%20%28single-precision%29)))

(fn ConstructionScript)

(fn AddAmount
  (params (Amount :type Integer))
  (bind _returnvalue (|(Amount+{C4E82756-4006-A9F1-557E-F6B4098F85CC}) Amount))
  (LocalVariables|SetTemp _returnvalue)
  (if (> _returnvalue (Variables|Stats|GetMaxAmount))
    (Variables|Stats|SetCurrentAmount (Variables|Stats|GetMaxAmount))
    (return (|({E3F90D68-4A14-513F-B724-ABA383A05AA1}-{F6393D17-4B27-6D75-DC3A-398AFF084108})))
    (else
      (Variables|Stats|SetCurrentAmount _returnvalue)
      (return 0))))

(fn SetAmount
  (params (Amount :type Integer))
  (Variables|Stats|SetCurrentAmount (Math|Integer|Clamp(Integer) Amount 1 (Variables|Stats|GetMaxAmount))))

(fn GetID
  (return (Default|GetIDfromObject (Subsystems|GetBPItemManager) self)))

(fn GetName
  (return (Variables|Stats|GetName)))

(fn GetDescription
  (return ""))

(fn GetRarityName
  (return (.Name (Utilities|GetClassDefaults (Variables|Stats|GetRarity)))))

(fn GetRarityOrderRule
  (return (.ComesBefore (Utilities|GetClassDefaults (Variables|Stats|GetRarity)))))

(fn GetRarityShader
  (return (.CustomShader (Utilities|GetClassDefaults (Variables|Stats|GetRarity)))))

(fn GetRarityDisplayWidget
  (return (.CustomDisplayWidget (Utilities|GetClassDefaults (Variables|Stats|GetRarity)))))

(fn GetCurrentAmount
  (return (Variables|Stats|GetCurrentAmount)))

(fn GetCalculatedWeight
  (return (|({C4E82756-4006-A9F1-557E-F6B4098F85CC}*{431CDD66-4FC4-03F4-1903-6BB559049F09}))))

(fn EqualsItemType
  (params (Not :type Boolean) (ItemType :type E_ItemType%20Enum :default "NewEnumerator7"))
  (if Not
    (return (Utilities|Enum|NotEqual(Enum) (Variables|Stats|GetItemType) ItemType))
    (else
      (return (Utilities|Enum|Equal(Enum) ItemType (Variables|Stats|GetItemType))))))

(fn IsFull
  (params (Not :type Boolean))
  (if Not
    (return (|({C4E82756-4006-A9F1-557E-F6B4098F85CC}=={F6393D17-4B27-6D75-DC3A-398AFF084108})))
    (else
      (return (|({C4E82756-4006-A9F1-557E-F6B4098F85CC}<{F6393D17-4B27-6D75-DC3A-398AFF084108}))))))

(fn SerializeCustomData
  (return 0))

(fn DeserializeItem
  (params (CustomData :type Array%20of%20Json%20Object%20Wrapper%20Structures)))

(fn Consume)