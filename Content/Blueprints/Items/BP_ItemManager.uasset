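; Item manager that builds registries of items, rarities and sort methods from DataTables on initialization.
; It provides lookups by ID or class and random picks, and orders rarities by each class's ComesBefore default.
; It also tracks toggleable, swappable sort methods, signalling changes.
; Sorting runs native-style predicate sorts through constructed comparator objects, with a second pass breaking ties when several methods are selected.
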(event `self.OnInitialize`
  (`self.SetupItems`)
  (`self.SetupSortMethods`)
  (`self.SetupRarities`))

(fn `CompareBySortMethod`
  (params (SortMethod :type "/Game/Blueprints/Inventory/BP_BaseSortMethod Class Reference") (A :type "/Game/Blueprints/Items/BP_BaseItem Object Reference") (B :type "/Game/Blueprints/Items/BP_BaseItem Object Reference"))
  (returns (Result :type Integer))
  (bind _returnvalue (`|GenericCreateObject` SortMethod))
  (return (`/Game/Blueprints/Inventory/BP_BaseSortMethod.Compare` _returnvalue A B)))

(fn `ConvertToItemArray`
  (params (ObjectArray :type "Array of Actor Object Reference"))
  (returns (ItemArray :type "Array of /Game/Blueprints/Items/BP_BaseItem Object Reference"))
  (locals (TempItemArray :type "Array of /Game/Blueprints/Items/BP_BaseItem Object Reference"))
  (bind _tempitemarray (`local.TempItemArray`))
  (for _array_element ObjectArray
    (bind _asbp_base_item (cast `/Game/Blueprints/Items/BP_BaseItem` _array_element))
    (`KismetArrayLibrary.Array_Add` _tempitemarray _asbp_base_item))
  (return _tempitemarray))

(fn `EqualIDs`
  (params (First :type "/Game/Blueprints/Items/S_ItemID Structure") (Second :type "/Game/Blueprints/Items/S_ItemID Structure"))
  (returns (equal :type Boolean))
  (return (and (`KismetStringLibrary.EqualEqual_StrStr` First_Source_2_D068BC2646C20B574D12DCBE5B6001E8 Second_Source_2_D068BC2646C20B574D12DCBE5B6001E8) (== First_ID_6_EC225C914E6EFFD1E516448773E2C340 Second_ID_6_EC225C914E6EFFD1E516448773E2C340))))

(fn `GetIDFromClass`
  (params (Item :type "/Game/Blueprints/Items/BP_BaseItem Class Reference"))
  (returns (ID :type "/Game/Blueprints/Items/S_ItemID Structure"))
  (for _array_element (`self.ItemRegistry`)
    (if (== Item (`.Item_10_360F4E6D4AACEC9BA74C6B95B047ED1D` (break `/Game/Blueprints/Items/S_ItemIDPair` _array_element)))
      (return (break `/Game/Blueprints/Items/S_ItemIDPair` _array_element))))
  (return (make `/Game/Blueprints/Items/S_ItemID` "Vanilla")))

(fn `GetIDFromObject`
  (params (Item :type "/Game/Blueprints/Items/BP_BaseItem Object Reference"))
  (returns (ID :type "/Game/Blueprints/Items/S_ItemID Structure"))
  (return (`self.GetIDFromClass` (`GameplayStatics.GetObjectClass` Item))))

(fn `GetIndexOfSortMethod`
  (params (SortMethod :type "/Game/Blueprints/Inventory/BP_BaseSortMethod Class Reference"))
  (returns (Index :type Integer))
  (for (_array_element _array_index) (`self.SortedSortRegistry`)
    (if (== SortMethod (break `/Game/Blueprints/Inventory/S_SortMethod` _array_element))
      (return _array_index))))

(fn `GetItem`
  (params (ID :type "/Game/Blueprints/Items/S_ItemID Structure"))
  (returns (Item :type "/Game/Blueprints/Items/BP_BaseItem Class Reference"))
  (for _array_element (`self.ItemRegistry`)
    (if (`self.EqualIDs` (break `/Game/Blueprints/Items/S_ItemIDPair` _array_element) ID)
      (return (`.Item_10_360F4E6D4AACEC9BA74C6B95B047ED1D` (break `/Game/Blueprints/Items/S_ItemIDPair` _array_element)))))
  (return null))

(fn `GetPossibleSortingMethods`
  (returns (PossibleSortMethods :type "Array of /Game/Blueprints/Inventory/S_SortMethod Structure"))
  (locals (SortMethods :type "Array of /Game/Blueprints/Inventory/S_SortMethod Structure") (VisibleSortMethods :type "Array of /Game/Blueprints/Inventory/S_SortMethod Structure"))
  (bind _sortmethods (`local.SortMethods`))
  (for _array_element (`self.SortRegistry`)
    (if (`.Status_4_2359B64B4789E18873ABC39563E218EC` (break `/Game/Blueprints/Inventory/S_SortMethod` _array_element))
      (`KismetArrayLibrary.Array_Add` _sortmethods (make `/Game/Blueprints/Inventory/S_SortMethod` (break `/Game/Blueprints/Inventory/S_SortMethod` _array_element) (`.Status_4_2359B64B4789E18873ABC39563E218EC` (break `/Game/Blueprints/Inventory/S_SortMethod` _array_element))))))
  (if (`KismetArrayLibrary.Array_IsEmpty` _sortmethods)
    (return (`self.SortRegistry`))
    (else
      (for _array_element_2 (`self.SortRegistry`)
        (if (`self.IsPossibleSortMethod` _array_element_2 (`local.SortMethods`))
          (`KismetArrayLibrary.Array_Add` (`local.VisibleSortMethods`) _array_element_2)))
      (return (`local.VisibleSortMethods`)))))

(fn `GetRandomItem`
  (returns (Item :type "/Game/Blueprints/Items/BP_BaseItem Class Reference"))
  (return (`.Item_10_360F4E6D4AACEC9BA74C6B95B047ED1D` (break `/Game/Blueprints/Items/S_ItemIDPair` (`KismetArrayLibrary.Array_Random` (`self.ItemRegistry`))))))

(fn `GetRandomItemID`
  (returns (ID :type "/Game/Blueprints/Items/S_ItemID Structure"))
  (return (break `/Game/Blueprints/Items/S_ItemIDPair` (`KismetArrayLibrary.Array_Random` (`self.ItemRegistry`)))))

(fn `GetSelectedSortMethods`
  (returns (SelectedSortMethods :type "Array of Integer"))
  (locals (Temp :type "Array of Integer"))
  (bind _temp (`local.Temp`))
  (for _array_element (`self.SortRegistry`)
    (if (`.Status_4_2359B64B4789E18873ABC39563E218EC` (break `/Game/Blueprints/Inventory/S_SortMethod` _array_element))
      (`KismetArrayLibrary.Array_Add` _temp (`self.GetIndexOfSortMethod` (break `/Game/Blueprints/Inventory/S_SortMethod` _array_element)))))
  (return _temp))

(fn `InternalFirstComparison`
  (params (A :type "Actor Object Reference") (B :type "Actor Object Reference") (SortMethod :type Integer))
  (returns (Result :type Boolean))
  (locals (FirstItem :type "/Game/Blueprints/Items/BP_BaseItem Object Reference") (SecondItem :type "/Game/Blueprints/Items/BP_BaseItem Object Reference"))
  (bind _output_sortmethod (break `/Game/Blueprints/Inventory/S_SortMethod` (`|GetArrayItem` (`self.SortedSortRegistry`) (`local.SortMethod`))))
  (`|ExecutionSequence`
    (:`then_0`
      (`|ExecutionSequence`
        (:`then_0`
          (bind _asbp_base_item (cast `/Game/Blueprints/Items/BP_BaseItem` A))
          (set `local.FirstItem` _asbp_base_item))
        (:`then_1`
          (bind _asbp_base_item_2 (cast `/Game/Blueprints/Items/BP_BaseItem` B))
          (set `local.SecondItem` _asbp_base_item_2))
        (:`then_2`
          (bind _result (`self.CompareBySortMethod` _output_sortmethod (`local.FirstItem`) (`local.SecondItem`)))
          (`self.ReadResult` _result
            (:`<`
              (return true))))))
    (:`then_1`
      (return false))))

(fn `InternalSecondComparison`
  (params (A :type "Actor Object Reference") (B :type "Actor Object Reference") (SortMethods :type "Array of Integer (by ref)") (Reverse :type Boolean))
  (returns (Result :type Boolean))
  (locals (FirstItem :type "/Game/Blueprints/Items/BP_BaseItem Object Reference") (SecondItem :type "/Game/Blueprints/Items/BP_BaseItem Object Reference"))
  (bind _sortmethods (`local.SortMethods`))
  (bind _output_sortmethod (break `/Game/Blueprints/Inventory/S_SortMethod` (`|GetArrayItem` (`self.SortedSortRegistry`) (`|GetArrayItem` (`local.SortMethods`)))))
  (`|ExecutionSequence`
    (:`then_0`
      (`|ExecutionSequence`
        (:`then_0`
          (bind _asbp_base_item (cast `/Game/Blueprints/Items/BP_BaseItem` A))
          (set `local.FirstItem` _asbp_base_item))
        (:`then_1`
          (bind _asbp_base_item_2 (cast `/Game/Blueprints/Items/BP_BaseItem` B))
          (set `local.SecondItem` _asbp_base_item_2))
        (:`then_2`
          (bind _result (`self.CompareBySortMethod` _output_sortmethod (`local.FirstItem`) (`local.SecondItem`)))
          (`self.ReadResult` _result
            (:`<`
              (if (not (`local.Reverse`))
                (return true)))
            (:`==`
              (for _index (range 1 (+ (`KismetArrayLibrary.Array_LastIndex` _sortmethods) 1))
                (bind _output_sortmethod_2 (break `/Game/Blueprints/Inventory/S_SortMethod` (`|GetArrayItem` (`self.SortedSortRegistry`) (`|GetArrayItem` _sortmethods _index))))
                (bind _result_2 (`self.CompareBySortMethod` _output_sortmethod_2 (`local.FirstItem`) (`local.SecondItem`)))
                (`self.ReadResult` _result_2
                  (:`<`
                    (return true))
                  (:`>`
                    (return false)))))
            (:`>`
              (if (`local.Reverse`)
                (return true)))))))
    (:`then_1`
      (return false))))

(fn `IsPossibleSortMethod`
  (params (SortMethod :type "/Game/Blueprints/Inventory/S_SortMethod Structure") (SortMethodSelection :type "Array of /Game/Blueprints/Inventory/S_SortMethod Structure"))
  (returns (Possible :type Boolean))
  (for _array_element SortMethodSelection
    (if (== (break `/Game/Blueprints/Inventory/S_SortMethod` _array_element) (`.Tier` (defaults `Object` SortMethod_SortMethod_2_C24735D24F8F9CDCC798BBAD2CDBEFE0)))
      (return false)))
  (return true))

(fn `LoadItems`
  (params (Datatable :type "DataTable Object Reference"))
  (bind _outrownames (`DataTableFunctionLibrary.GetDataTableRowNames` Datatable))
  (for _array_element _outrownames
    (bind _returnvalue (`|GetDataTableRow` Datatable _array_element)
      (:`then`
        (`KismetArrayLibrary.Array_Add` (`self.ItemRegistry`) _returnvalue)))))

(fn `LoadRarities`
  (params (Datatable :type "DataTable Object Reference"))
  (bind _outrownames (`DataTableFunctionLibrary.GetDataTableRowNames` Datatable))
  (for _array_element _outrownames
    (bind _returnvalue (`|GetDataTableRow` Datatable _array_element)
      (:`then`
        (`KismetArrayLibrary.Array_Add` (`self.RarityRegistry`) (`.Rarity_2_677E8093411027FC0E8580B0A962A482` (break `/Game/Blueprints/Items/S_Rarity` _returnvalue)))))))

(fn `LoadSortMethods`
  (params (Datatable :type "DataTable Object Reference"))
  (bind _outrownames (`DataTableFunctionLibrary.GetDataTableRowNames` Datatable))
  (for _array_element _outrownames
    (bind _returnvalue (`|GetDataTableRow` Datatable _array_element)
      (:`then`
        (`KismetArrayLibrary.Array_Add` (`self.SortedSortRegistry`) _returnvalue))))
  (set `self.SortRegistry` (`self.SortedSortRegistry`)))

(fn `LowerRaritiy`
  (params (A :type "/Game/Blueprints/Items/BP_RarityBase Class Reference") (B :type "/Game/Blueprints/Items/BP_RarityBase Class Reference"))
  (returns (Result :type Boolean))
  (bind _rarityregistry (`self.RarityRegistry`))
  (return (< (`KismetArrayLibrary.Array_Find` _rarityregistry A) (`KismetArrayLibrary.Array_Find` _rarityregistry B))))

(fn `MatchesRarityList`
  (params (First :type "Array of /Game/Blueprints/Items/BP_RarityBase Class Reference") (Second :type "Array of /Game/Blueprints/Items/BP_RarityBase Class Reference"))
  (returns (Result :type Boolean))
  (locals (Inside :type Boolean))
  (for _array_element First
    (bind _output_get (set `local.Inside` false))
    (for _array_element_2 Second
      (if (== _array_element _array_element_2)
        (set `local.Inside` true)))
    (if (not _output_get)
      (return false)))
  (return true))

(fn `SetSortMethodStatus`
  (params (SortMethod :type "/Game/Blueprints/Inventory/BP_BaseSortMethod Class Reference") (Status :type Boolean))
  (for (_array_element _array_index) (`self.SortRegistry`)
    (if (== SortMethod (break `/Game/Blueprints/Inventory/S_SortMethod` _array_element))
      (`KismetArrayLibrary.Array_Set` (`self.SortRegistry`) _array_index (make `/Game/Blueprints/Inventory/S_SortMethod` (break `/Game/Blueprints/Inventory/S_SortMethod` _array_element) (`local.Status`)))
      (break)))
  (`self.OnSortChanged`))

(fn `SetupItems`
  (`self.LoadItems` "/Game/Data/Items/Ores.Ores")
  (`self.LoadItems` "/Game/Data/Items/Ingots.Ingots")
  (`self.LoadItems` "/Game/Data/Items/Resources.Resources"))

(fn `SetupRarities`
  (`self.LoadRarities` "/Game/Data/Rarities.Rarities")
  (`self.SortRarities`))

(fn `SetupSortMethods`
  (`self.LoadSortMethods` "/Game/Data/SortingMethods.SortingMethods"))

(fn `ShouldCreate`
  (returns (ReturnValue :type Boolean))
  (return true))

(fn `Sort`
  (params (UnsortedItems :type "Array of /Game/Blueprints/Items/BP_BaseItem Object Reference") (SelectedSortMethods :type "Array of Integer") (Reverse :type Boolean))
  (returns (SortedItems :type "Array of /Game/Blueprints/Items/BP_BaseItem Object Reference") (Sorted :type Boolean))
  (bind _selectedsortmethods (`local.SelectedSortMethods`))
  (bind _unsorteditems (`local.UnsortedItems`))
  (if (`KismetArrayLibrary.Array_IsNotEmpty` SelectedSortMethods)
    (`GameUtilities.PredicateSortActorItemsFirst` UnsortedItems (`|CreateDelegate` :!event `InternalFirstComparison`) (`local.SelectedSortMethods`) Reverse)
    (if (< (`KismetArrayLibrary.Array_Length` _selectedsortmethods) 2)
      (return (`local.UnsortedItems`) true)
      (else
        (`GameUtilities.PredicateSortActorItemsSecond` _unsorteditems (`|CreateDelegate` :!event `InternalSecondComparison`) _selectedsortmethods (`local.Reverse`))
        (return _unsorteditems true)))
    (else
      (return (`local.UnsortedItems`) false))))

(fn `SortRarities`
  (locals (SortedRarities :type "Array of /Game/Blueprints/Items/BP_RarityBase Class Reference") (Index :type Integer))
  (bind _sortedrarities (`local.SortedRarities`))
  (for _array_element (`self.RarityRegistry`)
    (if (`KismetArrayLibrary.Array_IsEmpty` (`local.SortedRarities`))
      (`KismetArrayLibrary.Array_Add` _sortedrarities _array_element)
      (else
        (set `local.Index` (`KismetArrayLibrary.Array_Length` _sortedrarities))
        (for (_array_element_2 _array_index) _sortedrarities
          (if (== _array_element_2 (`.ComesBefore` (defaults `Object` _array_element)))
            (set `local.Index` _array_index)))
        (`KismetArrayLibrary.Array_Insert` (`local.SortedRarities`) _array_element (`local.Index`)))))
  (set `self.RarityRegistry` (`local.SortedRarities`)))

(fn `SwapSorts`
  (params (A :type "/Game/Blueprints/Inventory/BP_BaseSortMethod Class Reference") (B :type "/Game/Blueprints/Inventory/BP_BaseSortMethod Class Reference"))
  (locals (FirstIndex :type Integer) (SecondIndex :type Integer))
  (bind _sortregistry (`self.SortRegistry`))
  (bind _firstindex (`local.FirstIndex`))
  (bind _secondindex (`local.SecondIndex`))
  (if (!= A B)
    (for (_array_element _array_index) _sortregistry
      (`|ExecutionSequence`
        (:`then_0`
          (if (== A (break `/Game/Blueprints/Inventory/S_SortMethod` _array_element))
            (set `local.FirstIndex` _array_index)))
        (:`then_1`
          (if (== (break `/Game/Blueprints/Inventory/S_SortMethod` _array_element) (`local.B`))
            (set `local.SecondIndex` _array_index)))))
    (if (!= _firstindex _secondindex)
      (`KismetArrayLibrary.Array_Swap` _sortregistry _firstindex _secondindex)
      (`self.OnSortChanged`))))