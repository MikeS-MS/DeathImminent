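; Slot-based, replicated inventory component that stores item actors in a fixed-size array, spawned or attached to its owner.
; Adding fills existing stacks before free slots, and sorting merges stacks, then orders them through BPItemManager.
; Server events route add, transfer, drop and sort requests; transfers and drops check the passed item data against current slots.
; Changes and OnRep fire an OnChange notification, and items serialize by ID, slot, amount and custom data.
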(event EventBeginPlay
  (Networking|SwitchHasAuthority
    (:Authority
      (Setup|Setup))))

(event EventEndPlay
  (params (EndPlayReason :type EEndPlayReason%20Enum :default "Destroyed"))
  (if (Utilities|Enum|NotEqual(Enum) EndPlayReason "Quit")
    (Setup|ClearItems)))

(event Custom|Server_AddItemFromID
  (params (ID :type S%20Item%20ID%20Structure) (Amount :type Integer))
  (Operations|Items|AddItemfromID ID Amount))

(event Custom|Server_DropOnOtherItem
  (params (TargetInventory :type BP%20Inventory%20Object%20Reference) (DroppedItemIndex :type S%20Item%20Server%20Check%20Data%20Structure) (DroppedItemInventory :type BP%20Inventory%20Object%20Reference) (DroppedOnItemIndex :type S%20Item%20Server%20Check%20Data%20Structure))
  (Operations|Items|DroponOtherItem TargetInventory DroppedItemIndex DroppedItemInventory DroppedOnItemIndex))

(event Custom|Server_AddItemFromInventory
  (params (TargetInventory :type BP%20Inventory%20Object%20Reference) (Inventory :type BP%20Inventory%20Object%20Reference) (Index :type S%20Item%20Server%20Check%20Data%20Structure))
  (Operations|Items|AddItemfromInventory TargetInventory Inventory Index))

(event Custom|Server_SortItems
  (params (TargetInventory :type BP%20Inventory%20Object%20Reference) (SortMethodOrder :type Array%20of%20Integers) (Reverse :type Boolean))
  (Operations|Sorting|SortItems TargetInventory SortMethodOrder Reverse))

(fn SetItem
  (params (Index :type Integer) (Item :type BP%20Base%20Item%20Object%20Reference))
  (bind _returnvalue (Components|GetOwner))
  (Utilities|IsValid Item
    (:Is%20Valid
      (Actor|SetOwner Item _returnvalue)
      (Transformation|AttachActorToActor Item _returnvalue "None" "SnapToTarget" "SnapToTarget" "SnapToTarget" false)
      (Variables|/Game/Blueprints/Items/BP_BaseItem.BP_BaseItem_C|SetOwningInventory Item self))
    (:Is%20Not%20Valid
      _))
  (Utilities|Array|SetArrayElem (Variables|Default|GetItems) Index Item)
  (Default|CallOnChange))

(fn CreateItem
  (params (ItemClass :type BP%20Base%20Item%20Class%20Reference))
  (bind _returnvalue (Components|GetOwner))
  (bind _returnvalue_2 (Game|SpawnActorfromClass ItemClass (Math|Transform|MakeTransform "0, 0, 0" "0, 0, 0" "1.000000,1.000000,1.000000") "Undefined" _returnvalue self 0))
  (Transformation|AttachActorToActor _returnvalue_2 _returnvalue "None" "SnapToTarget" "SnapToTarget" "SnapToTarget" false)
  (return _returnvalue_2))

(fn TryAddNewStacks
  (params (Item :type BP%20Base%20Item%20Class%20Reference) (Amount :type Integer))
  (LocalVariables|SetAmountOfItem Amount)
  (LocalVariables|SetSlotIndex (Utility|Items|GetAvailableSlot))
  (while (|(({789D79A6-4EB3-50D4-BC07-B0A408B03568}>NegOne)&&({90AB95FD-4A60-18F6-8789-0ABEB050300C}>0)) -1)
    (bind _item (Operations|Items|CreateItem Item))
    (bind _output_get (LocalVariables|SetNewItem _item))
    (bind _amountleft (Default|AddAmount _output_get (LocalVariables|GetAmountOfItem)))
    (LocalVariables|SetAmountOfItem _amountleft)
    (Utilities|Array|SetArrayElem (Variables|Default|GetItems) (LocalVariables|GetSlotIndex) (LocalVariables|GetNewItem))
    (LocalVariables|SetSlotIndex (Utility|Items|GetAvailableSlot)))
  (return (LocalVariables|GetAmountOfItem)))

(fn FillExisting
  (params (Item :type BP%20Base%20Item%20Class%20Reference) (Amount :type Integer))
  (LocalVariables|SetTotalAmount Amount)
  (bind _output_get (LocalVariables|SetItemsFromInventory (Utility|Items|ItemExistsClass Item)))
  (for _array_element _output_get
    (if (|({14680DE5-42FF-8DD5-A0B8-4B808B7C532B}>0))
      (bind _amountleft (Default|AddAmount _array_element (LocalVariables|GetTotalAmount)))
      (bind _output_get_2 (LocalVariables|SetTempAmountLeft _amountleft))
      (if (|({9BBBAE5A-4373-B5AE-637C-5B80033D7501}!={14680DE5-42FF-8DD5-A0B8-4B808B7C532B}))
        (LocalVariables|SetTotalAmount _output_get_2))
      (else
        (return (LocalVariables|GetTotalAmount)))))
  (return (LocalVariables|GetTotalAmount)))

(fn AddItemfromID
  (params (ItemID :type S%20Item%20ID%20Structure) (Amount :type Integer))
  (Operations|Items|AddItemfromClass (Default|GetItem (Subsystems|GetBPItemManager) ItemID) Amount))

(fn AddItemfromClass
  (params (Item :type BP%20Base%20Item%20Class%20Reference) (Amount :type Integer))
  (Utilities|FlowControl|Sequence
    (:then_0
      (bind _amountleft (Operations|Items|FillExisting Item Amount))
      (LocalVariables|SetLocalAmountLeft _amountleft))
    (:then_1
      (if (|({DE28CEE2-4955-0826-D002-87B81A8AD201}>0))
        (bind _amountleft_2 (Operations|Items|TryAddNewStacks Item (LocalVariables|GetLocalAmountLeft)))
        (LocalVariables|SetLocalAmountLeft _amountleft_2)))
    (:then_2
      (Default|CallOnChange)
      (return (LocalVariables|GetLocalAmountLeft)))))

(fn AddItemfromInventory
  (params (TransferingItemInventory :type BP%20Inventory%20Object%20Reference) (TransferingItem :type S%20Item%20Server%20Check%20Data%20Structure))
  (bind _output_get (LocalVariables|SetItem (Utility|Items|GetItematIndex TransferingItemInventory (.index TransferingItem))))
  (Utilities|IsValid _output_get
    (:Is%20Valid
      (if (== (.item TransferingItem) _output_get)
        (Utilities|FlowControl|Sequence
          (:then_0
            (bind _amountleft (Operations|Items|FillExisting (Utilities|GetClass (LocalVariables|GetItem)) (Default|GetCurrentAmount (LocalVariables|GetItem))))
            (LocalVariables|SetAmountLeft _amountleft))
          (:then_1
            (if (|({144E0EE9-49DA-9A40-5220-A4BFF0EEE8B8}>0))
              (Default|SetAmount (LocalVariables|GetItem) (LocalVariables|GetAmountLeft))
              (bind _output_get_2 (LocalVariables|SetSlotIndex (Utility|Items|GetAvailableSlot)))
              (if (> _output_get_2 -1)
                (Operations|Items|SetItem _output_get_2 (LocalVariables|GetItem))
                (Operations|Items|SetItem TransferingItemInventory (.index TransferingItem) :!label _label))
              (else
                (goto _label)))))))))

(fn ItemExistsID
  (params (Item :type S%20Item%20ID%20Structure))
  (return (Utility|Items|ItemExistsClass (Default|GetItem (Subsystems|GetBPItemManager) Item))))

(fn ItemExistsClass
  (params (Item :type BP%20Base%20Item%20Class%20Reference))
  (bind _inventoryitems (LocalVariables|GetInventoryItems))
  (for _array_element (Variables|Default|GetItems)
    (Utilities|IsValid _array_element
      (:Is%20Valid
        (if (== (Utilities|GetClass _array_element) Item)
          (Utilities|Array|Add _inventoryitems _array_element)))))
  (return _inventoryitems))

(fn ItemExistsObject
  (params (Item :type BP%20Base%20Item%20Object%20Reference))
  (bind _inventoryitems (LocalVariables|GetInventoryItems))
  (for _array_element (Variables|Default|GetItems)
    (Utilities|IsValid _array_element
      (:Is%20Valid
        (if (== (Utilities|GetClass _array_element) (Utilities|GetClass Item))
          (Utilities|Array|Add _inventoryitems 0)))))
  (return _inventoryitems))

(fn GetItems
  (return (Variables|Default|GetItems)))

(fn GetAvailableSlot
  (for (_array_element _array_index) (Variables|Default|GetItems)
    (Utilities|IsValid _array_element
      (:Is%20Not%20Valid
        (return _array_index))))
  (return -1))

(fn GetIndexOfItem
  (params (Item :type BP%20Base%20Item%20Object%20Reference))
  (return (Utilities|Array|FindItem (Variables|Default|GetItems) Item)))

(fn GetItematIndex
  (params (Index :type Integer))
  (return (Utilities|Array|Get(acopy) (Variables|Default|GetItems) Index)))

(fn GetOnlyItems
  (bind _list (LocalVariables|GetList))
  (for _array_element (Variables|Default|GetItems)
    (Utilities|IsValid _array_element
      (:Is%20Valid
        (Utilities|Array|Add _list _array_element))))
  (return _list))

(fn ClearItems
  (bind _items (Variables|Default|GetItems))
  (for _array_element _items
    (Utilities|IsValid _array_element
      (:Is%20Valid
        (Actor|DestroyActor _array_element))))
  (Utilities|Array|Clear _items))

(fn SetItemsArraySize
  (bind _output_get (LocalVariables|SetLastIndex (- (Variables|Default|GetSlotCount) 1)))
  (for _index (range 0 _output_get)
    (Utilities|Array|Add (Variables|Default|GetItems) 0)))

(fn Setup
  (Setup|ClearItems)
  (Setup|SetItemsArraySize))

(fn RemoveItem
  (params (ItemIndex :type Integer))
  (bind _items (Variables|Default|GetItems))
  (Utilities|FlowControl|Sequence
    (:then_0
      (if (Utilities|Array|IsValidIndex _items ItemIndex)
        (Actor|DestroyActor (Utilities|Array|Get(acopy) _items ItemIndex))
        (Utilities|Array|SetArrayElem _items ItemIndex 0)))
    (:then_1
      (Default|CallOnChange))))

(fn SwapItems
  (params (First :type Integer) (Second :type Integer))
  (Utilities|Array|Swap (Variables|Default|GetItems) First Second))

(fn DroponOtherItem
  (params (DroppedItemData :type S%20Item%20Server%20Check%20Data%20Structure) (DroppedItemInventory :type BP%20Inventory%20Object%20Reference) (DroppedOnItemData :type S%20Item%20Server%20Check%20Data%20Structure))
  (bind _output_get (LocalVariables|SetInventoriesMatch (== DroppedItemInventory self)))
  (if _output_get
    (if (not (== (.index DroppedItemData) (.index DroppedOnItemData)))
      (bind _output_get_2 (LocalVariables|SetDroppedItem (Utility|Items|GetItematIndex DroppedItemInventory (.index DroppedItemData)) :!label _label))
      (bind _output_get_3 (LocalVariables|SetDroppedOnItem (Utility|Items|GetItematIndex (.index DroppedOnItemData))))
      (Utilities|IsValid _output_get_2
        (:Is%20Valid
          (if (|((ItemA==ItemB)&&(ItemAAmount==ItemBAmount)) (LocalVariables|GetDroppedItem) (.item DroppedItemData) (Default|GetCurrentAmount (LocalVariables|GetDroppedItem)) (.amount DroppedItemData))
            (if (== (LocalVariables|GetDroppedOnItem) (.item DroppedOnItemData))
              (Utilities|IsValid _output_get_3
                (:Is%20Valid
                  (if (== (Default|GetCurrentAmount (LocalVariables|GetDroppedOnItem)) (.amount DroppedOnItemData))
                    (if (Default|EqualIDs (Subsystems|GetBPItemManager) (.id DroppedItemData) (.id DroppedOnItemData))
                      (bind _amountleft (Default|AddAmount (LocalVariables|GetDroppedOnItem) (Default|GetCurrentAmount (LocalVariables|GetDroppedItem))))
                      (if (< _amountleft 1)
                        (Operations|Items|RemoveItem DroppedItemInventory (.index DroppedItemData))
                        (else
                          (Default|SetAmount (LocalVariables|GetDroppedItem) _amountleft)))
                      (else
                        (if (LocalVariables|GetInventoriesMatch) :!label _label_2
                          (Operations|Items|SwapItems (.index DroppedItemData) (.index DroppedOnItemData))
                          (Default|CallOnChange)
                          (else
                            (Operations|Items|SetItem (.index DroppedOnItemData) (LocalVariables|GetDroppedItem))
                            (Operations|Items|SetItem DroppedItemInventory (.index DroppedItemData) (LocalVariables|GetDroppedOnItem))))))))
                (:Is%20Not%20Valid
                  (goto _label_2))))))))
    (else
      (goto _label))))

(fn StackItems
  (for (_array_element _array_index) (Variables|Default|GetItems)
    (Utilities|IsValid _array_element
      (:Is%20Valid
        (bind _output_get (LocalVariables|SetFirstItem _array_element))
        (if (Default|IsFull _output_get true)
          (bind (_array_element_2 _array_index_2) (Utilities|Array|ForEachLoopwithBreak (Variables|Default|GetItems) :!label _label)
            (:LoopBody
              (Utilities|IsValid _array_element_2
                (:Is%20Valid
                  (bind _output_get_2 (LocalVariables|SetSecondItem _array_element_2))
                  (if (|(((ItemA==ItemB)&&(IndexA!=IndexB))&&Bool) (Utilities|GetClass (LocalVariables|GetFirstItem)) (Utilities|GetClass _output_get_2) _array_index_2 _array_index (Default|IsFull _output_get_2 true))
                    (bind _amountleft (Default|AddAmount (LocalVariables|GetSecondItem) (Default|GetCurrentAmount (LocalVariables|GetFirstItem))))
                    (bind _output_get_3 (LocalVariables|SetAmountLeft _amountleft))
                    (if (> _output_get_3 0)
                      (Default|SetAmount (LocalVariables|GetFirstItem) _output_get_3)
                      (else
                        (Operations|Items|RemoveItem _array_index)
                        (goto _label Break)))))))))))))

(fn FillRest
  (params (ItemArray :type Array%20of%20BP%20Base%20Item%20Object%20References))
  (bind _slotcount (Variables|Default|GetSlotCount))
  (if (== (Utilities|Array|Length ItemArray) _slotcount)
    _
    (else
      (bind _output_get (LocalVariables|SetFirstIndex (+ (Utilities|Array|LastIndex ItemArray) 1)))
      (bind _output_get_2 (LocalVariables|SetLastIndex (- _slotcount 1)))
      (for _index (range _output_get _output_get_2)
        (Utilities|Array|Add ItemArray 0))))
  (return ItemArray))

(fn SortItems
  (params (SelectedSortMethods :type Array%20of%20Integers) (Reverse :type Boolean))
  (Utilities|FlowControl|Sequence
    (:then_0
      (Operations|Items|StackItems)
      ;[1 1 1] TODO: Send a notification if false
      (bind (_sorteditems _sorted) (Default|Sort (Subsystems|GetBPItemManager) (Utility|Items|GetOnlyItems) SelectedSortMethods Reverse))
      (if _sorted
        (bind _filled (Operations|Sorting|FillRest _sorteditems))
        (Variables|Default|SetItems _filled)))
    (:then_1
      (Default|CallOnChange))))

(fn GetSerializedItem
  (params (Item :type BP%20Base%20Item%20Object%20Reference))
  (bind _customdata (Default|SerializeCustomData Item))
  (return (Utilities|Struct|MakeS_SerializedItem (Default|GetIDfromObject (Subsystems|GetBPItemManager) Item) (Utility|Items|GetIndexOfItem Item) (Default|GetCurrentAmount Item) _customdata)))

(fn SerializeItems
  (params (All :type Boolean) (ItemSelection :type Array%20of%20Integers))
  (bind _items (Variables|Default|GetItems))
  (bind _tempitems (LocalVariables|GetTempItems))
  (bind _tempitems_2 (LocalVariables|GetTempItems))
  (if All
    (for _array_element _items
      (Utilities|Array|Add _tempitems (Serialization|GetSerializedItem _array_element)))
    (return _tempitems)
    (else
      (for _array_element_2 ItemSelection
        (Utilities|Array|Add _tempitems_2 (Serialization|GetSerializedItem (Utilities|Array|Get(acopy) _items _array_element_2))))
      (return _tempitems_2))))

(fn DeserializeItems
  (params (SerializedItems :type Array%20of%20S%20Serialized%20Item%20Structures))
  (for _array_element SerializedItems
    (bind _returnvalue (Game|SpawnActorfromClass (Default|GetItem (Subsystems|GetBPItemManager) (.id _array_element)) (Math|Transform|MakeTransform "0, 0, 0" "0, 0, 0" "1.000000,1.000000,1.000000") "Undefined" 0 self 0))
    (bind _output_get (LocalVariables|SetItem _returnvalue))
    (Default|SetAmount _output_get (.amount _array_element))
    (Default|DeserializeItem _output_get (.customdata _array_element))
    (Utilities|Array|SetArrayElem (Variables|Default|GetItems) (.index _array_element) (LocalVariables|GetItem)))
  (Default|CallOnChange))

(fn SendSortRequest
  (params (TargetInventory :type BP%20Inventory%20Object%20Reference) (Reverse :type Boolean))
  (CallFunction|ServerSortItems TargetInventory (Default|GetSelectedSortMethods (Subsystems|GetBPItemManager)) Reverse))

(fn OnRepItems
  (Default|CallOnChange))