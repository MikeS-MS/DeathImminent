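; Interactable is a base actor for objects that a Player can use while standing inside its Box trigger.
; On the authority, box overlaps track the overlapping Player, and Tick calls ActionOnOverlap every frame while that player's IsUsing is set.
; InitialSetup, ActionOnOverlap, OnTick and RemoteTick are empty hooks, splitting per-frame logic between server and remote instances, presumably for child Blueprints to override.
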(event `self.ReceiveBeginPlay`
  (`self.InitialSetup`))

(event `self.ReceiveTick`
  (params (DeltaSeconds :type "Float (single-precision)"))
  (`/Engine/EditorBlueprintResources/ActorMacros.Switch Has Authority` self
    (:`Authority`
      (bind _asplayer (cast `/Game/Blueprints/Player` (`self.OverlappingActor`))
        (:`then`
          (if (`/Game/Blueprints/Player.isUsing` _asplayer)
            (`self.ActionOnOverlap`)))
        (:`CastFailed`
          _))
      (`self.OnTick`))
    (:`Remote`
      (`self.RemoteTick`))))

(event `self.Box.OnComponentBeginOverlap`
  (params (OverlappedComponent :type "PrimitiveComponent Object Reference") (OtherActor :type "Actor Object Reference") (OtherComp :type "PrimitiveComponent Object Reference") (OtherBodyIndex :type Integer) (bFromSweep :type Boolean) (SweepResult :type "HitResult Structure (by ref)"))
  (`/Engine/EditorBlueprintResources/ActorMacros.Switch Has Authority` self
    (:`Authority`
      (bind _asplayer (cast `/Game/Blueprints/Player` OtherActor))
      (set `self.ActorInside` true)
      (set `self.OverlappingActor` _asplayer))))

(event `self.Box.OnComponentEndOverlap`
  (params (OverlappedComponent :type "PrimitiveComponent Object Reference") (OtherActor :type "Actor Object Reference") (OtherComp :type "PrimitiveComponent Object Reference") (OtherBodyIndex :type Integer))
  (`/Engine/EditorBlueprintResources/ActorMacros.Switch Has Authority` self
    (:`Authority`
      (set `self.ActorInside` false)
      (set `self.OverlappingActor` null))))

(fn `ActionOnOverlap`)

(fn `InitialSetup`)

(fn `OnTick`)

(fn `RemoteTick`)

(fn `UserConstructionScript`)