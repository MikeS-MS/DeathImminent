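; Game instance Blueprint that handles session invites and loads weapon part stats from a remotely hosted JSON file.
; An accepted session invite immediately joins that session with the first player controller.
; A setup event downloads the stats file into the project's Saved directory with a short timeout, then loads weapon parts from it on success.
; Download progress and failed results are not handled.
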(event `self.OnSessionInviteAccepted`
  (params (LocalPlayerNum :type Integer) (PersonInvited :type "BPUniqueNetId Structure") (SessionToJoin :type "BlueprintSessionResult Structure (by ref)"))
  (`JoinSessionCallbackProxy.JoinSession` (`GameplayStatics.GetPlayerController` 0) SessionToJoin))

(event `DownloadWeaponPartsStatsFile`
  (`FileToStorageDownloader.BP_DownloadFileToStorage` (`self.StatsFileURL`) (`KismetStringLibrary.Concat_StrStr` (`BlueprintPathsLibrary.ProjectSavedDir`) (`self.FilePathToSaveTo`)) 5.0 "application/json" (delegate `EventOnProgressUpdatedStatsFile`) (delegate `EventOnStatsDownloaded`)))

(event `EventOnProgressUpdatedStatsFile`
  (params (BytesReceived :type Integer) (ContentLength :type Integer)))

(event `EventOnStatsDownloaded`
  (params (Result :type "EDownloadToStorageResult Enum" :default "SuccessDownloading"))
  (switch `EDownloadToStorageResult` Result
    (:`SuccessDownloading`
      (`/Game/Blueprints/Dev/BP_Functionality.LoadWeaponPartsFromJson` (`KismetStringLibrary.Concat_StrStr` (`BlueprintPathsLibrary.ProjectSavedDir`) (`self.FilePathToSaveTo`))))))