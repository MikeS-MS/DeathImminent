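; BP_ItemManager is an item registry that maps source-qualified IDs to items.
; LoadItems appends each row of a given data table to the registry.
; Lookups scan it linearly in either direction, matching IDs on both source and number, and fall back to BP_BaseItem or a default Vanilla ID when nothing matches.
; It also returns a random item or item ID from the registry.
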(fn `EqualIDs`
  (params (First :type "/Game/Blueprints/Entities/Inventory/S_ItemID Structure") (Second :type "/Game/Blueprints/Entities/Inventory/S_ItemID Structure"))
  (returns (equal :type Boolean))
  (return (and (`KismetStringLibrary.EqualEqual_StrStr` First_Source_2_D068BC2646C20B574D12DCBE5B6001E8 Second_Source_2_D068BC2646C20B574D12DCBE5B6001E8) (== First_ID_6_EC225C914E6EFFD1E516448773E2C340 Second_ID_6_EC225C914E6EFFD1E516448773E2C340))))

(fn `GetID`
  (params (Item :type "/Game/Blueprints/Entities/Inventory/Items/BP_BaseItem Class Reference"))
  (returns (ID :type "/Game/Blueprints/Entities/Inventory/S_ItemID Structure"))
  (for _array_element (`self.ItemRegistry`)
    (if (== Item (`.Item_7_360F4E6D4AACEC9BA74C6B95B047ED1D` (break `/Game/Blueprints/Entities/Inventory/S_ItemIDPair` _array_element)))
      (return (break `/Game/Blueprints/Entities/Inventory/S_ItemIDPair` _array_element))))
  (return (make `/Game/Blueprints/Entities/Inventory/S_ItemID` "Vanilla")))

(fn `GetItem`
  (params (ID :type "/Game/Blueprints/Entities/Inventory/S_ItemID Structure"))
  (returns (Item :type "/Game/Blueprints/Entities/Inventory/Items/BP_BaseItem Class Reference"))
  (for _array_element (`self.ItemRegistry`)
    (if (`self.EqualIDs` (break `/Game/Blueprints/Entities/Inventory/S_ItemIDPair` _array_element) ID)
      (return (`.Item_7_360F4E6D4AACEC9BA74C6B95B047ED1D` (break `/Game/Blueprints/Entities/Inventory/S_ItemIDPair` _array_element)))))
  (return "/Game/Blueprints/Entities/Inventory/Items/BP_BaseItem.BP_BaseItem_C"))

(fn `GetRandomItem`
  (returns (Item :type "/Game/Blueprints/Entities/Inventory/Items/BP_BaseItem Class Reference"))
  (return (`.Item_7_360F4E6D4AACEC9BA74C6B95B047ED1D` (break `/Game/Blueprints/Entities/Inventory/S_ItemIDPair` (`KismetArrayLibrary.Array_Random` (`self.ItemRegistry`))))))

(fn `GetRandomItemID`
  (returns (ID :type "/Game/Blueprints/Entities/Inventory/S_ItemID Structure"))
  (return (break `/Game/Blueprints/Entities/Inventory/S_ItemIDPair` (`KismetArrayLibrary.Array_Random` (`self.ItemRegistry`)))))

(fn `LoadItems`
  (params (Datatable :type "DataTable Object Reference"))
  (bind _outrownames (`DataTableFunctionLibrary.GetDataTableRowNames` Datatable))
  (for _array_element _outrownames
    (bind _returnvalue (`|GetDataTableRow` Datatable _array_element)
      (:`then`
        (`KismetArrayLibrary.Array_Add` (`self.ItemRegistry`) _returnvalue)))))