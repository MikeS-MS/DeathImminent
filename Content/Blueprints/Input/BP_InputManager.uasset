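; BP_InputManager manages Enhanced Input mapping contexts for the local player, covering gameplay and UI action keybinds.
; When the controller spawns, a one-time setup adds both IMC_Player and IMC_UIActions at priority zero.
; Separate functions add or remove each context through the first player's Enhanced Input local player subsystem.
; ShouldCreate always returns true, so creation is never filtered.
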(event `ControllerSpawned`
  (`self._Setup`))

(fn `_AddMappingContext`
  (params (MappingContext :type "InputMappingContext Object Reference"))
  (`EnhancedInputSubsystemInterface.AddMappingContext` (pcsubsystem `EnhancedInputLocalPlayerSubsystem` (`GameplayStatics.GetPlayerControllerFromID` 0)) MappingContext 0 (struct)))

(fn `_RemoveMappingContext`
  (params (MappingContext :type "InputMappingContext Object Reference"))
  (`EnhancedInputSubsystemInterface.RemoveMappingContext` (pcsubsystem `EnhancedInputLocalPlayerSubsystem` (`GameplayStatics.GetPlayerController` 0)) MappingContext (struct)))

(fn `_Setup`
  (if (not (`self.Setup`))
    (`self.AddPlayerKeybinds`)
    (`self.AddUIActionKeybinds`)
    (set `self.Setup` true)))

(fn `AddPlayerKeybinds`
  (`self._AddMappingContext` "/Game/Blueprints/Input/Player/IMC_Player.IMC_Player"))

(fn `AddUIActionKeybinds`
  (`self._AddMappingContext` "/Game/Blueprints/Input/UI/IMC_UIActions.IMC_UIActions"))

(fn `RemovePlayerKeybinds`
  (`self._RemoveMappingContext` "/Game/Blueprints/Input/Player/IMC_Player.IMC_Player"))

(fn `RemoveUIActionKeybinds`
  (`self._RemoveMappingContext` "/Game/Blueprints/Input/UI/IMC_UIActions.IMC_UIActions"))

(fn `ShouldCreate`
  (returns (ReturnValue :type Boolean))
  (return true))