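; Player controller for the survivor that relays input to its possessed BP_Player, cached on BeginPlay.
; Movement, look, jump, run and use inputs pass through the HudStatus macro, which blocks them while the UI manager reports the HUD toggled; Aim is an empty stub.
; Back and Inventory bypass that gate and call the UI manager, with Inventory passing the player's inventory as payload.
; OnLoadPlayer stores the character data from the save object.
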(event `self.ReceiveBeginPlay`
  (bind _asbp_player (cast `/Game/Blueprints/Entities/Player/BP_Player` (`self.K2_GetPawn`)))
  (set `self.PossessedPlayer` _asbp_player))

(event `/Game/Blueprints/Serializing/BPI_Serializable.OnLoadPlayer`
  (params (PlayerSaveGameObject :type "/Game/Blueprints/Serializing/BP_PlayerSaveGame Object Reference"))
  (set `self.SavedCharacter` (`/Game/Blueprints/Serializing/BP_PlayerSaveGame.PlayerData` PlayerSaveGameObject)))

(event `InputAction|Aim`
  (params (Key :type "Key Structure"))
  (:`Pressed`
    (`self.HudStatus`
      (:`NotToggled`
        (`self.PossessedPlayer`
          (:`then`)
          (:`else`))))))

(event `InputAction|Use`
  (params (Key :type "Key Structure"))
  (:`Pressed`
    (`self.HudStatus`
      (:`NotToggled`
        (bind _possessedplayer (`self.PossessedPlayer`)
          (:`then`
            (`/Game/Blueprints/Entities/Player/BP_Player.InputUse` _possessedplayer))
          (:`else`))))))

(event `InputAction|Jump`
  (params (Key :type "Key Structure"))
  (:`Pressed`
    (`self.HudStatus`
      (:`NotToggled`
        (bind _possessedplayer (`self.PossessedPlayer`)
          (:`then`
            (`/Game/Blueprints/Entities/Player/BP_Player.InputJumpPressed` _possessedplayer))
          (:`else`)))))
  (:`Released`
    (`self.HudStatus`
      (:`NotToggled`
        (bind _possessedplayer_2 (`self.PossessedPlayer`)
          (:`then`
            (`/Game/Blueprints/Entities/Player/BP_Player.InputJumpReleased` _possessedplayer_2))
          (:`else`))))))

(event `InputAction|Run`
  (params (Key :type "Key Structure"))
  (:`Pressed`
    (`self.HudStatus`
      (:`NotToggled`
        (bind _possessedplayer (`self.PossessedPlayer`)
          (:`then`
            (`/Game/Blueprints/Entities/Player/BP_Player.InputRunPressed` _possessedplayer))
          (:`else`)))))
  (:`Released`
    (`self.HudStatus`
      (:`NotToggled`
        (bind _possessedplayer_2 (`self.PossessedPlayer`)
          (:`then`
            (`/Game/Blueprints/Entities/Player/BP_Player.InputRunReleased` _possessedplayer_2))
          (:`else`))))))

(event `InputAxis|Turn`
  (params (AxisValue :type "Float (single-precision)"))
  (`self.HudStatus`
    (:`NotToggled`
      (bind _possessedplayer (`self.PossessedPlayer`)
        (:`then`
          (`/Game/Blueprints/Entities/Player/BP_Player.InputTurnHorizontal` _possessedplayer AxisValue))
        (:`else`)))))

(event `InputAxis|LookUp`
  (params (AxisValue :type "Float (single-precision)"))
  (`self.HudStatus`
    (:`NotToggled`
      (bind _possessedplayer (`self.PossessedPlayer`)
        (:`then`
          (`/Game/Blueprints/Entities/Player/BP_Player.InputTurnVertical` _possessedplayer AxisValue))
        (:`else`)))))

(event `InputAxis|TurnRate`
  (params (AxisValue :type "Float (single-precision)"))
  (`self.HudStatus`
    (:`NotToggled`
      (bind _possessedplayer (`self.PossessedPlayer`)
        (:`then`
          (`/Game/Blueprints/Entities/Player/BP_Player.InputTurnRate` _possessedplayer AxisValue))
        (:`else`)))))

(event `InputAxis|LookUpRate`
  (params (AxisValue :type "Float (single-precision)"))
  (`self.HudStatus`
    (:`NotToggled`
      (bind _possessedplayer (`self.PossessedPlayer`)
        (:`then`
          (`/Game/Blueprints/Entities/Player/BP_Player.InputLookUpRate` _possessedplayer AxisValue))
        (:`else`)))))

(event `InputAxis|MoveForward`
  (params (AxisValue :type "Float (single-precision)"))
  (`self.HudStatus`
    (:`NotToggled`
      (bind _possessedplayer (`self.PossessedPlayer`)
        (:`then`
          (`/Game/Blueprints/Entities/Player/BP_Player.InputMoveForward` _possessedplayer AxisValue))
        (:`else`)))))

(event `InputAxis|MoveRight`
  (params (AxisValue :type "Float (single-precision)"))
  (`self.HudStatus`
    (:`NotToggled`
      (bind _possessedplayer (`self.PossessedPlayer`)
        (:`then`
          (`/Game/Blueprints/Entities/Player/BP_Player.InputMoveSideways` _possessedplayer AxisValue))
        (:`else`)))))

(event `InputAction|Back`
  (params (Key :type "Key Structure"))
  (:`Pressed`
    (`/Game/Blueprints/UI/BP_UIManager.OnBackPressed` (subsystem `/Game/Blueprints/UI/BP_UIManager`))))

(event `InputAction|Inventory`
  (params (Key :type "Key Structure"))
  (:`Pressed`
    (`/Game/Blueprints/UI/BP_UIManager.OpenMenu` (subsystem `/Game/Blueprints/UI/BP_UIManager`) (make `/Game/Blueprints/UI/S_MenuID` "Vanilla" "Inventory") (`/Game/Blueprints/Entities/Player/BP_Player.Inventory` (`self.PossessedPlayer`)) true)))

(fn `UserConstructionScript`)