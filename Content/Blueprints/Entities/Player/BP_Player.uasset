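; First-person multiplayer player character with armed view, sprinting, interaction and grid block editing.
; Enhanced Input drives movement, while eye line traces target grid breaking or placement, offset along the view direction, and gate look-at interactables.
; Held interactables take priority, with use results routed to local success or failure callbacks.
; Server events set RepNotify rotation and running state; GameInstance handles hub and mission loading, and saves load into Inventory.
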(event `self.ReceiveBeginPlay`
  ;[1 1 1] Setup
  (`|ExecutionSequence`
    (:`then_0`
      (bind _asbp_game_instance (cast `/Game/Blueprints/BP_GameInstance` (`GameplayStatics.GetGameInstance`)))
      (set `self.GameInstance` _asbp_game_instance))
    (:`then_1`
      (cast `/Game/Blueprints/GameModes/BP_HubGameState` (`GameplayStatics.GetGameState`))
      (`self.OnJoinHub`))))

(event `Interact_Old`
  (bind _pickedupinteractible (`self.PickedUpInteractible`))
  (bind _interactable (`self.Interactable`))
  (bind (_hitresult _hit) (`self.GetPointAtEyes` (`self.InteractionDistance`)))
  ;[1 1 1] Interaction
  (`/Engine/EditorBlueprintResources/StandardMacros.IsValid` _pickedupinteractible
    (:`Is Valid`
      (`self.CallEventsOnInteractable` _pickedupinteractible))
    (:`Is Not Valid`
      (`/Engine/EditorBlueprintResources/StandardMacros.IsValid` _interactable
        (:`Is Valid`
          (if (`/Game/Blueprints/Environment/Interactable/BP_BaseInteractable.RequiresToLookAt` _interactable)
            (if (and (== (`/Game/Blueprints/Environment/Interactable/BP_BaseInteractable.ComponentToHit` _interactable) (`.HitComponent` (`GameplayStatics.BreakHitResult` _hitresult))) _hit)
              (`self.CallEventsOnInteractable` _interactable :!label _label))
            (else
              (goto _label))))))))

(event `Server_Turn`
  (set `self.ControlRotation` (`self.GetControlRotation`)))

(event `Server_LookUp`
  (set `self.ControlRotation` (`self.GetControlRotation`)))

(event `Server_SetRunning`
  (set `self.IsRunning` true))

(event `Server_SetWalking`
  (set `self.IsRunning` false))

(event `Local_OnPlayerUseSuccess`
  (params (Interactable :type "/Game/Blueprints/Environment/Interactable/BP_BaseInteractable Object Reference"))
  (`/Engine/EditorBlueprintResources/StandardMacros.IsValid` Interactable
    (:`Is Valid`
      (`/Game/Blueprints/Environment/Interactable/BP_BaseInteractable.Local_OnPlayerUseSuccess` Interactable self))))

(event `Local_OnPlayerUseFailed`
  (params (Interactable :type "/Game/Blueprints/Environment/Interactable/BP_BaseInteractable Object Reference"))
  (`/Engine/EditorBlueprintResources/StandardMacros.IsValid` Interactable
    (:`Is Valid`
      (`/Game/Blueprints/Environment/Interactable/BP_BaseInteractable.Local_OnPlayerUseFailed` Interactable self))))

(event `OnJoinHub`
  (bind _gameinstance (`self.GameInstance`)
    (:`then`
      (`/Game/Blueprints/BP_GameInstance.LoadPlayerHub` _gameinstance self))
    (:`else`)))

(event `OnJoinMission`
  (bind _gameinstance (`self.GameInstance`)
    (:`then`
      (`/Game/Blueprints/BP_GameInstance.LoadPlayerMission` _gameinstance self))
    (:`else`)))

(event `/Game/Blueprints/Serializing/BPI_Serializable.OnLoadPlayer`
  (params (PlayerSaveGameObject :type "/Game/Blueprints/Serializing/BP_PlayerSaveGame Object Reference"))
  (`/Game/Blueprints/Serializing/BPI_Serializable.OnLoadPlayer` (`self.Inventory`) PlayerSaveGameObject))

(event `EnhancedInput|/Game/Blueprints/Input/Player/Actions/IA_Move`
  (params (ActionValue :type "Vector2D Structure") (ElapsedSeconds :type "Float (double-precision)") (TriggeredSeconds :type "Float (double-precision)") (InputAction :type "InputAction Object Reference" :default "/Game/Blueprints/Input/Player/Actions/IA_Move.IA_Move"))
  (:`Triggered`
    (`self.AddMovementInput` (`self.GetActorRightVector`) ActionValue_X)
    (`self.AddMovementInput` (`self.GetActorForwardVector`) ActionValue_Y)))

(event `EnhancedInput|/Game/Blueprints/Input/Player/Actions/IA_Look`
  (params (ActionValue :type "Vector2D Structure") (ElapsedSeconds :type "Float (double-precision)") (TriggeredSeconds :type "Float (double-precision)") (InputAction :type "InputAction Object Reference" :default "/Game/Blueprints/Input/Player/Actions/IA_Look.IA_Look"))
  (:`Triggered`
    (`self.AddControllerYawInput` ActionValue_X)
    (`self.AddControllerPitchInput` ActionValue_Y)))

(event `EnhancedInput|/Game/Blueprints/Input/Player/Actions/IA_Jump`
  (params (ActionValue :type Boolean) (ElapsedSeconds :type "Float (double-precision)") (TriggeredSeconds :type "Float (double-precision)") (InputAction :type "InputAction Object Reference" :default "/Game/Blueprints/Input/Player/Actions/IA_Jump.IA_Jump"))
  (:`Triggered`
    (`self.Jump`))
  (:`Completed`
    (`self.StopJumping`)))

(event `EnhancedInput|/Game/Blueprints/Input/Player/Actions/IA_Interact`
  (params (ActionValue :type Boolean) (ElapsedSeconds :type "Float (double-precision)") (TriggeredSeconds :type "Float (double-precision)") (InputAction :type "InputAction Object Reference" :default "/Game/Blueprints/Input/Player/Actions/IA_Interact.IA_Interact"))
  (:`Triggered`
    (`self.Interact_Old`)))

(event `EnhancedInput|/Game/Blueprints/Input/Player/Actions/IA_Attack`
  (params (ActionValue :type Boolean) (ElapsedSeconds :type "Float (double-precision)") (TriggeredSeconds :type "Float (double-precision)") (InputAction :type "InputAction Object Reference" :default "/Game/Blueprints/Input/Player/Actions/IA_Attack.IA_Attack"))
  (bind (_hitresult _hit _direction) (`self.GetPointAtEyes` (`self.InteractionDistance`)))
  (:`Triggered`
    (if _hit
      (`GridModifyingComponent.BreakFromGridTest` (`self.GridModifying`) (+ (`.Location` (`GameplayStatics.BreakHitResult` _hitresult)) (* _direction (`self.Penetration`)))))))

(event `EnhancedInput|/Game/Blueprints/Input/Player/Actions/IA_PlaceBlock`
  (params (ActionValue :type Boolean) (ElapsedSeconds :type "Float (double-precision)") (TriggeredSeconds :type "Float (double-precision)") (InputAction :type "InputAction Object Reference" :default "/Game/Blueprints/Input/Player/Actions/IA_PlaceBlock.IA_PlaceBlock"))
  (bind (_hitresult _hit _direction) (`self.GetPointAtEyes` (`self.InteractionDistance`)))
  (:`Triggered`
    (if _hit
      (`GridModifyingComponent.AddToGridMultipleTest` (`self.GridModifying`) (+ (`.Location` (`GameplayStatics.BreakHitResult` _hitresult)) (* _direction (* (`self.Penetration`) -1.0))) (`self.TempBlocksEdit`)))))

(fn `CallEventsOnInteractable`
  (params (Interactable :type "/Game/Blueprints/Environment/Interactable/BP_BaseInteractable Object Reference"))
  (bind _success (`/Game/Blueprints/Environment/Interactable/BP_BaseInteractable.Server_OnPlayerUse` Interactable self))
  (if _success
    (`self.Local_OnPlayerUseSuccess` Interactable)
    (else
      (`self.Local_OnPlayerUseFailed` Interactable))))

(fn `GetPointAtEyes`
  (params (Distance :type "Float (double-precision)"))
  (returns (HitResult :type "HitResult Structure") (Hit :type Boolean) (Direction :type "Vector Structure"))
  (bind _camera (`self.Camera`))
  (bind _returnvalue (`SceneComponent.GetForwardVector` _camera))
  (bind _returnvalue_2 (`SceneComponent.K2_GetComponentLocation` _camera))
  (bind (_outhit _returnvalue_3) (`KismetSystemLibrary.LineTraceSingleForObjects` :`Start` _returnvalue_2 :`End` (+ _returnvalue_2 (* _returnvalue Distance)) :`ObjectTypes` (`|MakeArray` "ObjectTypeQuery1" "ObjectTypeQuery2" :!type "EObjectTypeQuery Enum") :`bTraceComplex` true :`DrawTime` 1.0))
  (return _outhit _returnvalue_3 _returnvalue))

(fn `GetPointsAtEyes`
  (params (Range :type "Float (double-precision)"))
  (returns (HitResult :type "Array of HitResult Structure") (Hit :type Boolean))
  (bind _returnvalue (`SceneComponent.K2_GetComponentLocation` (`self.Camera`)))
  (bind (_outhits _returnvalue_2) (`KismetSystemLibrary.LineTraceMultiForObjects` _returnvalue (+ _returnvalue (* (`self.GetActorForwardVector`) Range)) (`|MakeArray` "ObjectTypeQuery1" "ObjectTypeQuery2" "ObjectTypeQuery3" "ObjectTypeQuery4" :!type "EObjectTypeQuery Enum") true (`|MakeArray` self :!type "Actor Object Reference")))
  (return _outhits _returnvalue_2))

(fn `InputRunPressed`
  (`self.SetRunning`)
  (`self.Server_SetRunning`))

(fn `InputRunReleased`
  (`self.SetNotRunning`)
  (`self.Server_SetWalking`))

(fn `OnRep_ControlRotation`
  (`self.K2_SetActorRotation` (`self.ControlRotation`) true))

(fn `OnRep_IsRunning`
  (`self.UpdateRunning`))

(fn `SetNotRunning`
  (set `CharacterMovementComponent.MaxWalkSpeed` (`self.DefaultMS`) (`self.CharacterMovement`)))

(fn `SetRunning`
  (set `CharacterMovementComponent.MaxWalkSpeed` (* (`self.SprintMultiplier`) (`self.DefaultMS`)) (`self.CharacterMovement`)))

(fn `SetSteamID`
  (params (ID :type String))
  (set `self.SteamID` ID))

(fn `UpdateRunning`
  (if (`self.IsRunning`)
    (`self.SetRunning`)
    (else
      (`self.SetNotRunning`))))

(fn `UserConstructionScript`
  (`SceneComponent.K2_AttachToComponent` (`self.Gun`) (`self.Arms`) "GripPoint" "SnapToTarget" "SnapToTarget" "SnapToTarget" true))