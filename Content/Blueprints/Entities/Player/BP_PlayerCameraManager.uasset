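; BP_PlayerCameraManager glides itself to a requested location and rotation, apparently to move the player's camera between views.
; SetMoveToLocation stores the target transform and starts movement, which Tick eases with VInterpTo and RInterpTo at a shared speed.
; Once both match the target, it stops and fires the OnReachedTargetLocation dispatcher.
; BeginPlay caches a BP_Player reference, which the movement logic does not use.
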(event `self.ReceiveBeginPlay`
  (bind _asbp_player (cast `/Game/Blueprints/Entities/Player/BP_Player` (`GameplayStatics.GetPlayerCharacter` 0)))
  (bind _output_get (set `self.PlayerRef` _asbp_player)))

(event `self.ReceiveTick`
  (params (DeltaSeconds :type "Float (single-precision)"))
  (bind _returnvalue (`self.K2_GetActorLocation`))
  (bind _returnvalue_2 (`self.K2_GetActorRotation`))
  (bind _targetlocation (`self.TargetLocation`))
  (bind _speed (`self.Speed`))
  (bind _targetrotation (`self.TargetRotation`))
  (if (`self.StartMoving`)
    (`self.K2_SetActorLocation` (`KismetMathLibrary.VInterpTo` _returnvalue _targetlocation DeltaSeconds _speed))
    (`self.K2_SetActorRotation` (`KismetMathLibrary.RInterpTo` _returnvalue_2 _targetrotation DeltaSeconds _speed))
    (if (and (== _returnvalue _targetlocation) (== _returnvalue_2 _targetrotation))
      (set `self.StartMoving` false)
      (`self.OnReachedTargetLocation`))))

(fn `SetMoveToLocation`
  (params (TargetLocation :type "Vector Structure") (TargetRotation :type "Rotator Structure"))
  (set `self.TargetLocation` TargetLocation)
  (set `self.TargetRotation` TargetRotation)
  (set `self.StartMoving` true))

(fn `UserConstructionScript`)