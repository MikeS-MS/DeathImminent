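; Slot-based inventory that stores each item stack as a spawned item actor, with BP_BaseItem placeholders for empty slots.
; Adding by ID, class or source inventory tops up matching stacks before filling empty slots; drops merge, split or swap.
; Sorting merges stacks, predicate-sorts by ID, name or weight, then pads empty slots.
; Events wrap these operations and signal OnChange; player load only rebuilds empty slots, as LoadItems is an unused stub.
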(event `self.ReceiveBeginPlay`)

(event `Event_OnChange`
  (`self.OnChange`))

(event `Event_AddItemFromID`
  (params (ID :type "/Game/Blueprints/Entities/Inventory/S_ItemID Structure") (Amount :type Integer))
  (`self.AddItemFromID` ID Amount))

(event `Event_AddItemFromInventory`
  (params (Inventory :type "/Game/Blueprints/Entities/Inventory/BP_Inventory Object Reference") (Index :type Integer))
  (`self.AddItemFromInventory` Inventory Index))

(event `Event_DropOnOtherItem`
  (params (DroppedIndex :type Integer) (DroppedOnIndex :type Integer) (Half :type Boolean))
  (`self.DropOnOtherItem` DroppedIndex DroppedOnIndex Half))

(event `Event_SortItems`
  (params (SortMethod :type "/Game/Blueprints/Entities/Inventory/E_SortMethod Enum" :default "NewEnumerator0") (Inverse :type Boolean))
  (`self.SortItems` SortMethod Inverse))

(event `Server_SetupEvent`
  (`self.Setup`))

(event `/Game/Blueprints/Serializing/BPI_Serializable.OnLoadPlayer`
  (params (PlayerSaveGameObject :type "/Game/Blueprints/Serializing/BP_PlayerSaveGame Object Reference"))
  (`self.Server_SetupEvent`))

(fn `AddItemFromClass`
  (params (Item :type "/Game/Blueprints/Entities/Inventory/Items/BP_BaseItem Class Reference") (Amount :type Integer))
  (`|ExecutionSequence`
    (:`then_0`
      (bind _amountleft (`self.FillExisting` Item Amount))
      (if (> _amountleft 0)
        (`self.TryAddNewStacks` Item _amountleft)))
    (:`then_1`
      (`self.Event_OnChange`))))

(fn `AddItemFromID`
  (params (ItemID :type "/Game/Blueprints/Entities/Inventory/S_ItemID Structure") (Amount :type Integer))
  (bind _itemmanager (`/Game/Blueprints/BPML_StandardMacros.GetItemManager`)
    (:`Found`
      (bind _item (`/Game/Blueprints/BP_ItemManager.GetItem` _itemmanager ItemID))
      (`self.AddItemFromClass` _item Amount))))

(fn `AddItemFromInventory`
  (params (Inventory :type "/Game/Blueprints/Entities/Inventory/BP_Inventory Object Reference") (Index :type Integer))
  (`|ExecutionSequence`
    (:`then_0`
      (bind _item (`self.GetItemAtIndex` Inventory Index))
      (if (`|EnumInequality` (`/Game/Blueprints/Entities/Inventory/Items/BP_BaseItem.ItemType` _item) "NewEnumerator7")
        (bind _returnvalue (`GameplayStatics.GetObjectClass` _item))
        (bind _amountleft (`self.FillExisting` _returnvalue (`/Game/Blueprints/Entities/Inventory/Items/BP_BaseItem.CurrentAmount` _item)))
        (if (> _amountleft 0)
          (bind _amountleft_2 (`self.TryAddNewStacks` _returnvalue _amountleft))
          (if (> _amountleft_2 0)
            (`/Game/Blueprints/Entities/Inventory/Items/BP_BaseItem.SetAmount` _item _amountleft_2)
            (else
              (`self.RemoveItem` Inventory Index))))))
    (:`then_1`
      (`self.Event_OnChange`))))

(fn `CheckEnoughSpace`
  (returns (Slot :type Integer))
  (for (_array_element _array_index) (`self.Items`)
    (if (`|EnumEquality` (`/Game/Blueprints/Entities/Inventory/Items/BP_BaseItem.ItemType` _array_element) "NewEnumerator7")
      (return _array_index)))
  (return -1))

(fn `ConvertToItemArray`
  (params (ActorArray :type "Array of Actor Object Reference"))
  (returns (ItemArray :type "Array of /Game/Blueprints/Entities/Inventory/Items/BP_BaseItem Object Reference"))
  (locals (TempItemArray :type "Array of /Game/Blueprints/Entities/Inventory/Items/BP_BaseItem Object Reference"))
  (bind _tempitemarray (`local.TempItemArray`))
  (for _array_element ActorArray
    (bind _asbp_base_item (cast `/Game/Blueprints/Entities/Inventory/Items/BP_BaseItem` _array_element))
    (`KismetArrayLibrary.Array_Add` _tempitemarray _asbp_base_item))
  (return _tempitemarray))

(fn `DropOnOtherItem`
  (params (DroppedIndex :type Integer) (DroppedOnIndex :type Integer) (Half :type Boolean))
  (locals (First :type "/Game/Blueprints/Entities/Inventory/Items/BP_BaseItem Object Reference") (Second :type "/Game/Blueprints/Entities/Inventory/Items/BP_BaseItem Object Reference") (HalfAmount :type Integer))
  (bind _droppedonindex (`local.DroppedOnIndex`))
  (bind _first (`local.First`))
  (bind _half (`local.Half`))
  (bind _first_2 (`local.First`))
  (bind _second (`local.Second`))
  (bind _currentamount (`/Game/Blueprints/Entities/Inventory/Items/BP_BaseItem.CurrentAmount` (`local.First`)))
  (bind _returnvalue (/ _currentamount 2))
  (if (!= DroppedIndex DroppedOnIndex)
    (bind _item (`self.GetItemAtIndex` DroppedIndex))
    (bind _item_2 (`self.GetItemAtIndex` DroppedOnIndex))
    (set `local.First` _item)
    (bind _output_get (set `local.Second` _item_2))
    (`|ExecutionSequence`
      (:`then_0`
        (bind _returnvalue_2 (`GameplayStatics.GetObjectClass` _item))
        (if (== _returnvalue_2 (`GameplayStatics.GetObjectClass` _item_2))
          (if (and (`/Game/Blueprints/Entities/Inventory/Items/BP_BaseItem.IsFull` _output_get) (`|EnumEquality` (`/Game/Blueprints/Entities/Inventory/Items/BP_BaseItem.ItemType` _item) "NewEnumerator7"))
            (`self.SwapItems` (`local.DroppedIndex`) (`local.DroppedOnIndex`) :!label _label)
            (elif _half
              (bind _output_get_2 (set `local.HalfAmount` _returnvalue))
              (bind _amountleft (`/Game/Blueprints/Entities/Inventory/Items/BP_BaseItem.AddAmount` _second _returnvalue))
              (if (> _amountleft 0)
                (`/Game/Blueprints/Entities/Inventory/Items/BP_BaseItem.SetAmount` _first_2 (+ _amountleft (- _currentamount _output_get_2))))
              (else
                (bind _amountleft_2 (`/Game/Blueprints/Entities/Inventory/Items/BP_BaseItem.AddAmount` _second _currentamount))
                (if (> _amountleft_2 0)
                  (`/Game/Blueprints/Entities/Inventory/Items/BP_BaseItem.SetAmount` _first_2 _amountleft_2)
                  (else
                    (`self.RemoveItem` (`local.DroppedIndex`)))))))
          (elif _half
            (if (`|EnumEquality` (`/Game/Blueprints/Entities/Inventory/Items/BP_BaseItem.ItemType` (`local.Second`)) "NewEnumerator7")
              (bind _returnvalue_3 (`|SpawnActorFromClass` _returnvalue_2 (`KismetMathLibrary.MakeTransform` (0.0 0.0 0.0)) "Undefined" "OverrideRootScale" null null))
              (`self.RemoveItem` _droppedonindex)
              (`KismetArrayLibrary.Array_Set` (`self.Items`) _droppedonindex _returnvalue_3)
              (`/Game/Blueprints/Entities/Inventory/Items/BP_BaseItem.SetAmount` _returnvalue_3 _returnvalue)
              (`/Game/Blueprints/Entities/Inventory/Items/BP_BaseItem.SetAmount` _first (- (`/Game/Blueprints/Entities/Inventory/Items/BP_BaseItem.CurrentAmount` _first) _returnvalue)))
            (else
              (goto _label)))))
      (:`then_1`
        (`self.Event_OnChange` :!label _label_2)))
    (else
      (goto _label_2))))

(fn `FillExisting`
  (params (Item :type "/Game/Blueprints/Entities/Inventory/Items/BP_BaseItem Class Reference") (Amount :type Integer))
  (returns (AmountLeft :type Integer))
  (locals (TotalAmount :type Integer))
  (bind _output_get (set `local.TotalAmount` Amount))
  (bind _itemsfrominventory (`self.ItemExistsClass` Item))
  (for _array_element _itemsfrominventory
    (if (> _output_get 0)
      (bind _amountleft (`/Game/Blueprints/Entities/Inventory/Items/BP_BaseItem.AddAmount` _array_element _output_get))
      (bind _output_get_2 (set `local.TotalAmount` _amountleft))
      (else
        (return _output_get_2))))
  (return _output_get_2))

(fn `FillRest`
  (params (Items :type "Array of /Game/Blueprints/Entities/Inventory/Items/BP_BaseItem Object Reference"))
  (returns (Filled :type "Array of /Game/Blueprints/Entities/Inventory/Items/BP_BaseItem Object Reference"))
  (bind _slotcount (`self.SlotCount`))
  (if (not (== (`KismetArrayLibrary.Array_Length` Items) _slotcount))
    (for _ (range (+ (`KismetArrayLibrary.Array_LastIndex` Items) 1) _slotcount)
      (bind _returnvalue (`|SpawnActorFromClass` "/Game/Blueprints/Entities/Inventory/Items/BP_BaseItem.BP_BaseItem_C" (`KismetMathLibrary.MakeTransform` (0.0 0.0 0.0)) "Undefined" "OverrideRootScale" null null))
      (`KismetArrayLibrary.Array_Add` Items _returnvalue)))
  (return Items))

(fn `GetItemAtIndex`
  (params (Index :type Integer))
  (returns (Item :type "/Game/Blueprints/Entities/Inventory/Items/BP_BaseItem Object Reference"))
  (return (`|GetArrayItem` (`self.Items`) Index)))

(fn `GetItems`
  (returns (Items :type "Array of /Game/Blueprints/Entities/Inventory/Items/BP_BaseItem Object Reference"))
  (return (`self.Items`)))

(fn `GetOnlyItems`
  (returns (Items :type "Array of /Game/Blueprints/Entities/Inventory/Items/BP_BaseItem Object Reference"))
  (locals (List :type "Array of /Game/Blueprints/Entities/Inventory/Items/BP_BaseItem Object Reference"))
  (bind _list (`local.List`))
  (for _array_element (`self.Items`)
    (if (`|EnumInequality` (`/Game/Blueprints/Entities/Inventory/Items/BP_BaseItem.ItemType` _array_element) "NewEnumerator7")
      (`KismetArrayLibrary.Array_Add` _list _array_element)
      (else
        (`Actor.K2_DestroyActor` _array_element))))
  (return _list))

(fn `ItemExistsClass`
  (params (Item :type "/Game/Blueprints/Entities/Inventory/Items/BP_BaseItem Class Reference"))
  (returns (ItemsFromInventory :type "Array of /Game/Blueprints/Entities/Inventory/Items/BP_BaseItem Object Reference"))
  (locals (InventoryItems :type "Array of /Game/Blueprints/Entities/Inventory/Items/BP_BaseItem Object Reference") (ItemManager :type "/Game/Blueprints/BP_ItemManager Object Reference"))
  (bind _inventoryitems (`local.InventoryItems`))
  (for _array_element (`self.Items`)
    (if (== (`GameplayStatics.GetObjectClass` _array_element) Item)
      (`KismetArrayLibrary.Array_Add` _inventoryitems _array_element)))
  (return _inventoryitems))

(fn `ItemExistsID`
  (params (Item :type "/Game/Blueprints/Entities/Inventory/S_ItemID Structure"))
  (returns (ItemsFromInventory :type "Array of /Game/Blueprints/Entities/Inventory/Items/BP_BaseItem Object Reference"))
  (locals (InventoryItems :type "Array of /Game/Blueprints/Entities/Inventory/Items/BP_BaseItem Object Reference") (ItemManager :type "/Game/Blueprints/BP_ItemManager Object Reference"))
  (bind _inventoryitems (`local.InventoryItems`))
  (bind _itemmanager (`/Game/Blueprints/BPML_StandardMacros.GetItemManager`)
    (:`Found`
      (bind _item (`/Game/Blueprints/BP_ItemManager.GetItem` _itemmanager Item))
      (for _array_element (`self.Items`)
        (if (== (`GameplayStatics.GetObjectClass` _array_element) _item)
          (`KismetArrayLibrary.Array_Add` _inventoryitems _array_element)))
      (return _inventoryitems))))

(fn `ItemExistsObject`
  (params (Item :type "/Game/Blueprints/Entities/Inventory/Items/BP_BaseItem Object Reference"))
  (returns (ItemsFromInventory :type "Array of /Game/Blueprints/Entities/Inventory/Items/BP_BaseItem Object Reference"))
  (locals (InventoryItems :type "Array of /Game/Blueprints/Entities/Inventory/Items/BP_BaseItem Object Reference"))
  (bind _inventoryitems (`local.InventoryItems`))
  (for _array_element (`self.Items`)
    (if (== (`GameplayStatics.GetObjectClass` _array_element) (`GameplayStatics.GetObjectClass` Item))
      (`KismetArrayLibrary.Array_Add` _inventoryitems _array_element)))
  (return _inventoryitems))

(fn `LesserString`
  (params (A :type String) (B :type String))
  (returns (Lesser :type Boolean))
  (for _index (range (+ (`KismetMathLibrary.Min` (`KismetStringLibrary.Len` A) (`KismetStringLibrary.Len` B)) 1))
    (bind _returnvalue (`KismetStringLibrary.GetCharacterAsNumber` A _index))
    (bind _returnvalue_2 (`KismetStringLibrary.GetCharacterAsNumber` B _index))
    (if (< _returnvalue _returnvalue_2)
      (return true)
      (elif (not (== _returnvalue _returnvalue_2))
        (return false))))
  (return false))

(fn `LoadItems`
  (params (PlayerSaveGame :type "/Game/Blueprints/Serializing/BP_PlayerSaveGame Object Reference")))

(fn `RemoveItem`
  (params (ItemIndex :type Integer))
  (bind _items (`self.Items`))
  (`|ExecutionSequence`
    (:`then_0`
      (if (`KismetArrayLibrary.Array_IsValidIndex` _items ItemIndex)
        (bind _item (`self.GetItemAtIndex` ItemIndex))
        (`Actor.K2_DestroyActor` _item)
        (bind _returnvalue (`|SpawnActorFromClass` "/Game/Blueprints/Entities/Inventory/Items/BP_BaseItem.BP_BaseItem_C" (`KismetMathLibrary.MakeTransform` (0.0 0.0 0.0)) "Undefined" "OverrideRootScale" null null))
        (`KismetArrayLibrary.Array_Set` _items ItemIndex _returnvalue)))
    (:`then_1`
      (`self.OnChange`))))

(fn `Setup`
  (bind _items (`self.Items`))
  (for _array_element _items
    (`Actor.K2_DestroyActor` _array_element))
  (`KismetArrayLibrary.Array_Clear` _items)
  (for _ (range (`self.SlotCount`))
    (bind _returnvalue (`|SpawnActorFromClass` "/Game/Blueprints/Entities/Inventory/Items/BP_BaseItem.BP_BaseItem_C" (`KismetMathLibrary.MakeTransform` (0.0 0.0 0.0)) "Undefined" "OverrideRootScale" null null))
    (`KismetArrayLibrary.Array_Add` _items _returnvalue)))

(fn `SortByID`
  (params (A :type "Actor Object Reference") (B :type "Actor Object Reference"))
  (returns (Result :type Boolean))
  (bind _asbp_base_item (cast `/Game/Blueprints/Entities/Inventory/Items/BP_BaseItem` A))
  (bind _asbp_base_item_2 (cast `/Game/Blueprints/Entities/Inventory/Items/BP_BaseItem` B))
  (bind (_id_source _id_id) (break `/Game/Blueprints/Entities/Inventory/S_ItemID` (`/Game/Blueprints/Entities/Inventory/Items/BP_BaseItem.GetID` _asbp_base_item)))
  (bind (_id_source_2 _id_id_2) (break `/Game/Blueprints/Entities/Inventory/S_ItemID` (`/Game/Blueprints/Entities/Inventory/Items/BP_BaseItem.GetID` _asbp_base_item_2)))
  (bind _lesser (`self.LesserString` _id_source _id_source_2))
  (if _lesser
    (return _lesser)
    (else
      (bind _returnvalue (< _id_id _id_id_2))
      (if _returnvalue
        _
        (elif (== _id_id _id_id_2)
          (return (> (`/Game/Blueprints/Entities/Inventory/Items/BP_BaseItem.CurrentAmount` _asbp_base_item) (`/Game/Blueprints/Entities/Inventory/Items/BP_BaseItem.CurrentAmount` _asbp_base_item_2)))
          (else
            _)))
      (return _returnvalue))))

(fn `SortByName`
  (params (A :type "Actor Object Reference") (B :type "Actor Object Reference"))
  (returns (Result :type Boolean))
  (bind _asbp_base_item (cast `/Game/Blueprints/Entities/Inventory/Items/BP_BaseItem` A))
  (bind _asbp_base_item_2 (cast `/Game/Blueprints/Entities/Inventory/Items/BP_BaseItem` B))
  (bind _name (`/Game/Blueprints/Entities/Inventory/Items/BP_BaseItem.Name` _asbp_base_item))
  (bind _name_2 (`/Game/Blueprints/Entities/Inventory/Items/BP_BaseItem.Name` _asbp_base_item_2))
  (bind _lesser (`self.LesserString` _name _name_2))
  (if _lesser
    _
    (elif (`KismetStringLibrary.EqualEqual_StrStr` _name _name_2)
      (return (> (`/Game/Blueprints/Entities/Inventory/Items/BP_BaseItem.CurrentAmount` _asbp_base_item) (`/Game/Blueprints/Entities/Inventory/Items/BP_BaseItem.CurrentAmount` _asbp_base_item_2)))
      (else
        _)))
  (return _lesser))

(fn `SortByWeight`
  (params (A :type "Actor Object Reference") (B :type "Actor Object Reference"))
  (returns (Result :type Boolean))
  (bind _asbp_base_item (cast `/Game/Blueprints/Entities/Inventory/Items/BP_BaseItem` A))
  (bind _asbp_base_item_2 (cast `/Game/Blueprints/Entities/Inventory/Items/BP_BaseItem` B))
  (return (< (`/Game/Blueprints/Entities/Inventory/Items/BP_BaseItem.GetWeight` _asbp_base_item) (`/Game/Blueprints/Entities/Inventory/Items/BP_BaseItem.GetWeight` _asbp_base_item_2))))

(fn `SortItems`
  (params (Method :type "/Game/Blueprints/Entities/Inventory/E_SortMethod Enum" :default "NewEnumerator0") (Inverse :type Boolean))
  (locals (ItemArray :type "Array of /Game/Blueprints/Entities/Inventory/Items/BP_BaseItem Object Reference"))
  (bind _items (`self.GetOnlyItems`))
  (`self.StackItems`)
  (`|ExecutionSequence`
    (:`then_0`
      (switch `/Game/Blueprints/Entities/Inventory/E_SortMethod` Method
        (:`NewEnumerator0`
          (bind _returnvalue (`SortPluginBPLibrary.PredicateSortActor` _items (`|CreateDelegate` :!event `SortByID`) Inverse))
          (bind _itemarray (`self.ConvertToItemArray` _returnvalue))
          (set `local.ItemArray` _itemarray))
        (:`NewEnumerator1`
          (bind _returnvalue_2 (`SortPluginBPLibrary.PredicateSortActor` _items (`|CreateDelegate` :!event `SortByName`) Inverse))
          (bind _itemarray_2 (`self.ConvertToItemArray` _returnvalue_2))
          (set `local.ItemArray` _itemarray_2))
        (:`NewEnumerator2`
          (bind _returnvalue_3 (`SortPluginBPLibrary.PredicateSortActor` _items (`|CreateDelegate` :!event `SortByWeight`) Inverse))
          (bind _itemarray_3 (`self.ConvertToItemArray` _returnvalue_3))
          (set `local.ItemArray` _itemarray_3))))
    (:`then_1`
      (bind _filled (`self.FillRest` (`local.ItemArray`)))
      (set `self.Items` _filled))
    (:`then_2`
      (`self.Event_OnChange`))))

(fn `StackItems`
  (locals (FirstItem :type "/Game/Blueprints/Entities/Inventory/Items/BP_BaseItem Object Reference") (SecondItem :type "/Game/Blueprints/Entities/Inventory/Items/BP_BaseItem Object Reference"))
  (bind _items (`self.Items`))
  (for (_array_element _array_index) _items
    (bind _output_get (set `local.FirstItem` _array_element))
    (if (and (not (`/Game/Blueprints/Entities/Inventory/Items/BP_BaseItem.IsFull` _output_get)) (`|EnumInequality` (`/Game/Blueprints/Entities/Inventory/Items/BP_BaseItem.ItemType` _output_get) "NewEnumerator7"))
      (for (_array_element_2 _array_index_2) _items
        (bind _output_get_2 (set `local.SecondItem` _array_element_2))
        (if (and (== (`GameplayStatics.GetObjectClass` (`local.FirstItem`)) (`GameplayStatics.GetObjectClass` _output_get_2)) (!= _array_index_2 _array_index) (not (`/Game/Blueprints/Entities/Inventory/Items/BP_BaseItem.IsFull` _output_get_2)))
          (bind _amountleft (`/Game/Blueprints/Entities/Inventory/Items/BP_BaseItem.AddAmount` (`local.SecondItem`) (`/Game/Blueprints/Entities/Inventory/Items/BP_BaseItem.CurrentAmount` (`local.FirstItem`))))
          (if (> _amountleft 0)
            (`/Game/Blueprints/Entities/Inventory/Items/BP_BaseItem.SetAmount` (`local.FirstItem`) _amountleft)
            (else
              (`self.RemoveItem` _array_index))))))))

(fn `SwapItems`
  (params (First :type Integer) (Second :type Integer))
  (locals (Temp :type Boolean))
  (`KismetArrayLibrary.Array_Swap` (`self.Items`) First Second))

(fn `TryAddNewStacks`
  (params (Item :type "/Game/Blueprints/Entities/Inventory/Items/BP_BaseItem Class Reference") (Amount :type Integer))
  (returns (AmountLeft :type Integer))
  (locals (SlotIndex :type Integer) (AmountOfItem :type Integer))
  (bind _output_get (set `local.AmountOfItem` Amount))
  (bind _slot (`self.CheckEnoughSpace`))
  (bind _output_get_2 (set `local.SlotIndex` _slot))
  (while (and (> _output_get_2 -1) (> _output_get 0))
    (bind _item (`self.GetItemAtIndex` _output_get_2))
    (`/Engine/EditorBlueprintResources/StandardMacros.IsValid` _item
      (:`Is Valid`
        (`Actor.K2_DestroyActor` _item))
      (:`Is Not Valid`
        _))
    (bind _returnvalue (`|SpawnActorFromClass` Item (`KismetMathLibrary.MakeTransform` (0.0 0.0 0.0)) "Undefined" "OverrideRootScale" null null))
    (bind _amountleft (`/Game/Blueprints/Entities/Inventory/Items/BP_BaseItem.AddAmount` _returnvalue _output_get))
    (`KismetArrayLibrary.Array_Set` (`self.Items`) _output_get_2 _returnvalue)
    (set `local.AmountOfItem` _amountleft)
    (bind _slot_2 (`self.CheckEnoughSpace`))
    (set `local.SlotIndex` _slot_2))
  (return _output_get))