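; Base class for inventory items, holding a stackable amount with a maximum and a per-unit weight.
; AddAmount fills the stack and returns the overflow, SetAmount clamps between one and the maximum, and helpers report total weight and fullness.
; Consumability and description return false and empty as defaults for child items.
; GetID looks up the item's ID by its class through the item manager.
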(event `self.ReceiveBeginPlay`)

(event `self.ReceiveDestroyed`)

(fn `AddAmount`
  (params (Amount :type Integer))
  (returns (AmountLeft :type Integer))
  (locals (Temp :type Integer))
  (bind _maxamount (`self.MaxAmount`))
  (bind _returnvalue (+ Amount (`self.CurrentAmount`)))
  (bind _output_get (set `local.Temp` _returnvalue))
  (if (> _returnvalue _maxamount)
    (set `self.CurrentAmount` _maxamount)
    (return (- _output_get _maxamount))
    (else
      (set `self.CurrentAmount` _returnvalue)
      (return 0))))

(fn `CanBeConsumed`
  (returns (CanBeConsumed :type Boolean))
  (return false))

(fn `GetDescription`
  (returns (Description :type String))
  (return ""))

(fn `GetID`
  (returns (ID :type "/Game/Blueprints/Entities/Inventory/S_ItemID Structure"))
  (bind _itemmanager (`/Game/Blueprints/BPML_StandardMacros.GetItemManager`)
    (:`Found`
      (bind _id (`/Game/Blueprints/BP_ItemManager.GetID` _itemmanager (`GameplayStatics.GetObjectClass` self)))
      (return _id))))

(fn `GetWeight`
  (returns (Weight :type "Float (double-precision)"))
  (return (* (`self.CurrentAmount`) (`self.Weight`))))

(fn `IsFull`
  (returns (Full :type Boolean))
  (return (== (`self.CurrentAmount`) (`self.MaxAmount`))))

(fn `SetAmount`
  (params (Amount :type Integer))
  (set `self.CurrentAmount` (`KismetMathLibrary.Clamp` Amount 1 (`self.MaxAmount`))))

(fn `UserConstructionScript`)