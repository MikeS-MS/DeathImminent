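; Game instance that manages startup, sessions and save slots, loading item tables and world/player saves on Init.
; StartGame opens Hub solo or as an Advanced Sessions listen server; accepted invites join sessions.
; LoadPlayerHub restores players from fixed-name save slots.
; The server runs a hub autosave timer targeting SaveData, absent here, and saves on non-mission exit; SaveSlotsData writes only player data.
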(event `self.ReceiveInit`
  (bind _returnvalue (`|GenericCreateObject` "/Game/Blueprints/BP_ItemManager.BP_ItemManager_C" self))
  (`InstanceSubsystem.Load` (subsystem `InstanceSubsystem`) _returnvalue)
  (`/Game/Blueprints/BP_ItemManager.LoadItems` _returnvalue "/Game/Data/Items/Ores.Ores")
  (`/Game/Blueprints/BP_ItemManager.LoadItems` _returnvalue "/Game/Data/Items/Ingots.Ingots")
  (`/Game/Blueprints/BP_ItemManager.LoadItems` _returnvalue "/Game/Data/Items/Resources.Resources")
  ;[1 1 1] Test
  (`self.StartGameDemo`))

(event `self.OnSessionInviteAccepted`
  (params (LocalPlayerNum :type Integer) (PersonInvited :type "BPUniqueNetId Structure") (SessionToJoin :type "BlueprintSessionResult Structure (by ref)"))
  (`JoinSessionCallbackProxy.JoinSession` (`GameplayStatics.GetPlayerController` 0) SessionToJoin))

(event `Event On Hub Entered`
  (if (`KismetSystemLibrary.IsServer`)
    (bind _returnvalue (`KismetSystemLibrary.K2_SetTimer` self "SaveData" (`self.AutoSaveTime`) true))
    (set `self.AutoSaveTimer` _returnvalue)))

(event `Event On Hub Left`
  (params (Mission :type Boolean))
  (if (`KismetSystemLibrary.IsServer`)
    (`KismetSystemLibrary.K2_ClearAndInvalidateTimerHandle` (`self.AutoSaveTimer`))
    (if (not Mission)
      (`self.SaveSlotsData`))))

(event `LoadHubLevel`
  (params (Solo :type Boolean) (LoadedWorldData :type Boolean) (LoadedPlayerData :type Boolean))
  (`|ExecutionSequence`
    (:`then_0`
      (if (not Solo)
        (`CreateSessionCallbackProxyAdvanced.CreateAdvancedSession` :`PlayerController` (`GameplayStatics.GetPlayerController` 0) :`PublicConnections` 0 :`PrivateConnections` 4 :`bAllowJoinViaPresenceFriendsOnly` true :`bUsesStats` true
          (:`OnSuccess`
            (`GameplayStatics.OpenLevel` "Hub" true "listen")))
        (else
          (`GameplayStatics.OpenLevel` "Hub"))))))

(event `LoadPlayerHub`
  (params (Player :type "/Game/Blueprints/Entities/Player/BP_Player Object Reference"))
  (bind _playersavedataobject (`self.PlayerSaveDataObject`))
  (bind _playerdata_transform (break `/Game/Blueprints/Serializing/S_PlayerSaveData` (`/Game/Blueprints/Serializing/BP_PlayerSaveGame.PlayerData` _playersavedataobject)))
  (if (`/Game/Blueprints/Serializing/BP_PlayerSaveGame.Loaded` _playersavedataobject)
    (`Actor.K2_SetActorTransform` Player _playerdata_transform true true)
    (else
      (`/Game/Blueprints/Serializing/BPI_Serializable.OnLoadPlayer` Player (`self.PlayerSaveDataObject`)))))

(event `LoadPlayerMission`
  (params (Player :type "/Game/Blueprints/Entities/Player/BP_Player Object Reference")))

(fn `CreatePlayerSaveSlot`
  (bind _returnvalue (`GameplayStatics.CreateSaveGameObject` "/Game/Blueprints/Serializing/BP_PlayerSaveGame.BP_PlayerSaveGame_C"))
  (set `self.PlayerSaveDataObject` _returnvalue))

(fn `CreateWorldSaveSlot`
  (bind _returnvalue (`GameplayStatics.CreateSaveGameObject` "/Game/Blueprints/Serializing/BP_WorldSaveGame.BP_WorldSaveGame_C"))
  (set `self.WorldSaveDataObject` _returnvalue))

(fn `GetPlayerSaveSlotPath`
  (returns (Path :type String))
  (return (`KismetStringLibrary.Concat_StrStr` "Player/" "bruh" ".plr")))

(fn `GetWorldSaveSlotPath`
  (returns (Path :type String))
  (return (`KismetStringLibrary.Concat_StrStr` "Game/" "Current.wld")))

(fn `LoadOrCreatePlayerSave`
  (returns (Exists :type Boolean))
  (bind _returnvalue (`KismetStringLibrary.Concat_StrStr` (`KismetSystemLibrary.GetProjectSavedDirectory`) "Player"))
  (if (not (`BlueprintPathsLibrary.DirectoryExists` _returnvalue))
    (`FileHelperBPLibrary.MakeDirectory` _returnvalue))
  (bind _exists (`self.LoadPlayerSaveSlot`))
  (if _exists
    (return _exists)
    (else
      (`self.CreatePlayerSaveSlot`)
      (return _exists))))

(fn `LoadOrCreateWorldSave`
  (returns (Exists :type Boolean))
  (bind _returnvalue (`KismetStringLibrary.Concat_StrStr` (`KismetSystemLibrary.GetProjectSavedDirectory`) "Game"))
  (if (not (`BlueprintPathsLibrary.DirectoryExists` _returnvalue))
    (`FileHelperBPLibrary.MakeDirectory` _returnvalue))
  (bind _exists (`self.LoadWorldSaveSlot`))
  (if _exists
    (return _exists)
    (else
      (`self.CreateWorldSaveSlot`)
      (return _exists))))

(fn `LoadPlayerSaveSlot`
  (returns (Exists :type Boolean))
  (bind _path (`self.GetPlayerSaveSlotPath`))
  (bind _returnvalue (`GameplayStatics.DoesSaveGameExist` _path))
  (if _returnvalue
    (bind _returnvalue_2 (`GameplayStatics.LoadGameFromSlot` _path))
    (bind _asbp_player_save_game (cast `/Game/Blueprints/Serializing/BP_PlayerSaveGame` _returnvalue_2)
      (:`then`
        (set `self.PlayerSaveDataObject` _asbp_player_save_game)
        (return _returnvalue))
      (:`CastFailed`
        _)))
  (return _returnvalue))

(fn `LoadWorldSaveSlot`
  (returns (Exists :type Boolean))
  (bind _path (`self.GetWorldSaveSlotPath`))
  (bind _returnvalue (`GameplayStatics.DoesSaveGameExist` _path))
  (if _returnvalue
    (bind _returnvalue_2 (`GameplayStatics.LoadGameFromSlot` _path))
    (bind _asbp_world_save_game (cast `/Game/Blueprints/Serializing/BP_WorldSaveGame` _returnvalue_2)
      (:`then`
        (set `self.WorldSaveDataObject` _asbp_world_save_game)
        (return _returnvalue))
      (:`CastFailed`
        _)))
  (return _returnvalue))

(fn `SaveSlotsData`
  (bind _playersavedataobject (`self.PlayerSaveDataObject`))
  (`|ExecutionSequence`
    (:`then_1`
      (bind _asbp_player (cast `/Game/Blueprints/Entities/Player/BP_Player` (`GameplayStatics.GetPlayerCharacter` 0)))
      (`/Game/Blueprints/Serializing/BP_PlayerSaveGame.SavePlayer` _playersavedataobject _asbp_player)
      (bind _returnvalue (`GameplayStatics.SaveGameToSlot` _playersavedataobject (`self.GetPlayerSaveSlotPath`)))
      (if _returnvalue
        _))))

(fn `Start Game`
  (params (Solo :type Boolean))
  (bind _exists (`self.LoadOrCreateWorldSave`))
  (bind _exists_2 (`self.LoadOrCreatePlayerSave`))
  (`self.LoadHubLevel` Solo _exists _exists_2))

(fn `StartGameDemo`
  (`self.LoadOrCreateWorldSave`)
  (`self.LoadOrCreatePlayerSave`))