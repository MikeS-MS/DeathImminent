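; Sliding door Blueprint that moves a supplied mesh between closed and open positions.
; SetMeshComponent records the mesh's start location and derives the open location from its bounds and per-axis settings, with SetComponent offering size-based, custom or additive offsets.
; Tick moves the mesh toward the current target at constant speed on each axis.
; Toggle flips the direction only after the mesh reaches either end.
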(event `Event Function SetMeshComponent`
  (bind _mesh (`self.Mesh`))
  ;[1 1 1] SetUp where to consider the open location and where the close location of the given mesh.
  (bind _output_get (set `self.BeginLocation` (`SceneComponent.K2_GetComponentLocation` _mesh)))
  (bind _returnvalue (`SlidingDoor.SetUpPositions` (`self.X`) (`self.Y`) (`self.Z`) (`.BoxExtent` (`KismetSystemLibrary.GetComponentBounds` _mesh)) _output_get))
  (set `self.EndLocation` _returnvalue))

(event `self.ReceiveTick`
  (params (DeltaSeconds :type "Float (single-precision)"))
  (bind _endlocation (`self.EndLocation`))
  (bind _beginlocation (`self.BeginLocation`))
  (bind _returnvalue (`SceneComponent.K2_GetComponentLocation` (`self.Mesh`)))
  ;[1 1 1] Handle Door Opening/Closing
  (if (`self.Open`)
    (`self.CheckIfReachedTarget` DeltaSeconds _endlocation)
    (else
      (`self.CheckIfReachedTarget` DeltaSeconds _beginlocation)))
  (if (or (== _returnvalue _endlocation) (== _returnvalue _beginlocation))
    (set `self.FinishedAnimation` true)))

(fn `CheckIfReachedTarget`
  (params (DeltaTime :type "Float (double-precision)") (Target :type "Vector Structure"))
  (bind _returnvalue (`SceneComponent.K2_GetComponentLocation` (`self.Mesh`)))
  (if (!= _returnvalue Target)
    (bind _position (`self.GetFinalPosition` _returnvalue Target DeltaTime))
    (`SceneComponent.K2_SetWorldLocation` (`self.Mesh`) _position false false))
  (return))

(fn `GetFinalPosition`
  (params (CurrentPosition :type "Vector Structure (by ref)") (TargetPosition :type "Vector Structure (by ref)") (DeltaTime :type "Float (double-precision) (by ref)"))
  (returns (Position :type "Vector Structure"))
  (bind _scalarmove (`self.ScalarMove`))
  (return (`KismetMathLibrary.MakeVector` (`KismetMathLibrary.FInterpTo_Constant` (.x CurrentPosition) (.x TargetPosition) DeltaTime _scalarmove) (`KismetMathLibrary.FInterpTo_Constant` (.y CurrentPosition) (.y TargetPosition) DeltaTime _scalarmove) (`KismetMathLibrary.FInterpTo_Constant` (.z CurrentPosition) (.z TargetPosition) DeltaTime _scalarmove))))

(fn `SetComponent`
  (params (Axis :type "Float (double-precision)") (Size :type "Float (double-precision)") (MovePos :type "MovePosition Structure (by ref)"))
  (returns (OutAxis :type "Float (double-precision)"))
  (locals (TempAxis :type Boolean))
  (bind (_benablemoving _movedirection _benableadditive _additivemovevalue _bcustommovevalue _moveby) (break `MovePosition` MovePos))
  (return (+ Axis (* (+ (+ (* (* (`KismetMathLibrary.Conv_BoolToDouble` _benablemoving) Size) (`KismetMathLibrary.Conv_BoolToDouble` (not _bcustommovevalue))) (* (`KismetMathLibrary.Conv_BoolToDouble` _benableadditive) _additivemovevalue)) (* (`KismetMathLibrary.Conv_BoolToDouble` _bcustommovevalue) _moveby)) (`KismetMathLibrary.Conv_IntToDouble` _movedirection)))))

(fn `SetMeshComponent`
  (params (Mesh :type "StaticMeshComponent Object Reference (by ref)"))
  (set `self.Mesh` Mesh)
  (`self.Event Function SetMeshComponent`)
  (return))

(fn `Toggle`
  (if (`self.FinishedAnimation`)
    (set `self.Open` (not (`self.Open`)))
    (set `self.FinishedAnimation` false)))