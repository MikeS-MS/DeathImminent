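; BP_GameInputResolver translates gameplay input into actions on a referenced Player character.
; Press and release events drive jumping, running and interaction after validity checks, while use release does nothing.
; Axis events feed movement along the player's forward and right vectors and controller yaw and pitch, without validity checks.
; Running and look changes are applied locally and also sent through the player's Server-prefixed functions for networking.
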(event `self.OnJumpPress`
  (bind _player (`self.Player`))
  (`/Engine/EditorBlueprintResources/StandardMacros.IsValid` _player
    (:`Is Valid`
      (`Character.Jump` _player))))

(event `self.OnJumpRelease`
  (bind _player (`self.Player`))
  (`/Engine/EditorBlueprintResources/StandardMacros.IsValid` _player
    (:`Is Valid`
      (`Character.StopJumping` _player))))

(event `self.OnRunPress`
  (bind _player (`self.Player`))
  (`/Engine/EditorBlueprintResources/StandardMacros.IsValid` _player
    (:`Is Valid`
      (`/Game/Dev/Blueprints/Entities/Players/BP_Player.SetRunning` _player)
      (`/Game/Dev/Blueprints/Entities/Players/BP_Player.Server_SetRunning` _player))))

(event `self.OnRunRelease`
  (bind _player (`self.Player`))
  (`/Engine/EditorBlueprintResources/StandardMacros.IsValid` _player
    (:`Is Valid`
      (`/Game/Dev/Blueprints/Entities/Players/BP_Player.SetNotRunning` _player)
      (`/Game/Dev/Blueprints/Entities/Players/BP_Player.Server_SetWalking` _player))))

(event `self.OnUsePress`
  (bind _player (`self.Player`))
  (`/Engine/EditorBlueprintResources/StandardMacros.IsValid` _player
    (:`Is Valid`
      (`/Game/Dev/Blueprints/Entities/Players/BP_Player.Interact` _player))))

(event `self.OnUseRelease`
  (`/Engine/EditorBlueprintResources/StandardMacros.IsValid` (`self.Player`)))

(event `self.InputAxis MoveForward`
  (params (AxisValue :type "Float (single-precision)"))
  (bind _player (`self.Player`))
  (`Pawn.AddMovementInput` _player (`Actor.GetActorForwardVector` _player) AxisValue false))

(event `self.InputAxis MoveRight`
  (params (AxisValue :type "Float (single-precision)"))
  (bind _player (`self.Player`))
  (`Pawn.AddMovementInput` _player (`Actor.GetActorRightVector` _player) AxisValue false))

(event `self.InputAxis Turn`
  (params (`Axis Value` :type "Float (single-precision)"))
  (bind _player (`self.Player`))
  (`Pawn.AddControllerYawInput` _player `Axis Value`)
  (`/Game/Dev/Blueprints/Entities/Players/BP_Player.Server_Turn` _player `Axis Value`))

(event `self.InputAxis LookUp`
  (params (`Axis Value` :type "Float (single-precision)"))
  (bind _player (`self.Player`))
  (`Pawn.AddControllerPitchInput` _player `Axis Value`)
  (`/Game/Dev/Blueprints/Entities/Players/BP_Player.Server_LookUp` _player `Axis Value`))