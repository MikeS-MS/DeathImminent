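; BP_Item is a base Blueprint for interactable items in the environment, holding each item's display name, ID and image.
; Getter functions expose these fields, and GetInfo joins the name and ID into a single descriptive string.
; Image has a RepNotify handler, which is empty, and SetupInfo is an empty stub.
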(fn `GetDisplayName`
  (returns (Name :type Text))
  (return (`self.DisplayName`)))

(fn `GetImage`
  (returns (Image :type "Material Object Reference"))
  (return (`self.Image`)))

(fn `GetInfo`
  (returns (Info :type String))
  (return (`KismetStringLibrary.Concat_StrStr` (`KismetStringLibrary.Concat_StrStr` (`KismetStringLibrary.Concat_StrStr` (`KismetStringLibrary.Concat_StrStr` "(Name: " (`KismetTextLibrary.Conv_TextToString` (`self.DisplayName`))) ", ItemID: ") (`KismetStringLibrary.Conv_IntToString` (`self.ItemID`))) ")")))

(fn `GetItemID`
  (returns (ItemID :type Integer))
  (return (`self.ItemID`)))

(fn `OnRep_Image`)

(fn `SetupInfo`)