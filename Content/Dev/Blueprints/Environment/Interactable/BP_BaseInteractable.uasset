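; Base interactable actor that registers itself with any BP_Player overlapping its collision.
; Overlap begin and end fire server events on authority, which set or clear the player's Interactable reference, and local events for the locally controlled player.
; Local enter, leave and use success or failure events are empty hooks, and Server_OnPlayerUse returns true by default.
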(event `self.ReceiveBeginPlay`)

(event `self.ReceiveTick`
  (params (DeltaSeconds :type "Float (single-precision)")))

(event `self.Collision.OnComponentBeginOverlap`
  (params (OverlappedComponent :type "PrimitiveComponent Object Reference") (OtherActor :type "Actor Object Reference") (OtherComp :type "PrimitiveComponent Object Reference") (OtherBodyIndex :type Integer) (bFromSweep :type Boolean) (SweepResult :type "HitResult Structure (by ref)"))
  (bind _asbp_player (cast `/Game/Shipping/Blueprints/Entities/Players/BP_Player` OtherActor))
  (`|ExecutionSequence`
    (:`then_0`
      (`/Engine/EditorBlueprintResources/ActorMacros.Switch Has Authority`
        (:`Authority`
          (`self.Server_OnPlayerEnter` _asbp_player))))
    (:`then_1`
      (if (`Pawn.IsLocallyControlled` _asbp_player)
        (`self.Local_OnPlayerEnter` _asbp_player)))))

(event `self.Collision.OnComponentEndOverlap`
  (params (OverlappedComponent :type "PrimitiveComponent Object Reference") (OtherActor :type "Actor Object Reference") (OtherComp :type "PrimitiveComponent Object Reference") (OtherBodyIndex :type Integer))
  (bind _asbp_player (cast `/Game/Shipping/Blueprints/Entities/Players/BP_Player` OtherActor))
  (`|ExecutionSequence`
    (:`then_0`
      (`/Engine/EditorBlueprintResources/ActorMacros.Switch Has Authority`
        (:`Authority`
          (`self.Server_OnPlayerLeave` _asbp_player))))
    (:`then_1`
      (if (`Pawn.IsLocallyControlled` _asbp_player)
        (`self.Local_OnPlayerLeave` _asbp_player)))))

(event `Local_OnPlayerEnter`
  (params (Player :type "/Game/Shipping/Blueprints/Entities/Players/BP_Player Object Reference")))

(event `Local_OnPlayerLeave`
  (params (Player :type "/Game/Shipping/Blueprints/Entities/Players/BP_Player Object Reference")))

(event `Local_OnPlayerUseSuccess`
  (params (Player :type "/Game/Shipping/Blueprints/Entities/Players/BP_Player Object Reference")))

(event `Local_OnPlayerUseFailed`
  (params (Player :type "/Game/Shipping/Blueprints/Entities/Players/BP_Player Object Reference")))

(event `Server_OnPlayerEnter`
  (params (Player :type "/Game/Shipping/Blueprints/Entities/Players/BP_Player Object Reference"))
  (set `/Game/Shipping/Blueprints/Entities/Players/BP_Player.Interactable` self Player))

(event `Server_OnPlayerLeave`
  (params (Player :type "/Game/Shipping/Blueprints/Entities/Players/BP_Player Object Reference (by ref)"))
  (if (== (`/Game/Shipping/Blueprints/Entities/Players/BP_Player.Interactable` Player) self)
    (set `/Game/Shipping/Blueprints/Entities/Players/BP_Player.Interactable` null Player)))

(fn `OnRep_Collision`)

(fn `Server_OnPlayerUse`
  (params (Player :type "/Game/Shipping/Blueprints/Entities/Players/BP_Player Object Reference"))
  (returns (Status :type Boolean))
  (return true))

(fn `UserConstructionScript`)