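; Base movable interactable component that lets a player pick up and drop its owning actor.
; Server-side use toggles between attaching the owner to the player with collision off and detaching it in place.
; Pickup suspends the look-at requirement and registers itself as the player's held interactable; drop reverses both.
; The PickedUp RepNotify mirrors the collision state on clients.
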(fn `Drop`
  (params (Player :type "/Game/Dev/Blueprints/Entities/Players/BP_Player Object Reference"))
  (bind _returnvalue (`self.GetOwner`))
  (`Actor.K2_DetachFromActor` _returnvalue "KeepWorld" "KeepWorld" "KeepWorld")
  (`Actor.SetActorEnableCollision` _returnvalue true)
  (set `self.PickedUp` false)
  (set `self.RequiresToLookAt` (`self.BackupRequiresToLookAt`))
  (if (== (`/Game/Dev/Blueprints/Entities/Players/BP_Player.PickedUpInteractible` Player) self)
    (set `/Game/Dev/Blueprints/Entities/Players/BP_Player.PickedUpInteractible` null Player)))

(fn `OnRep_PickedUp`
  (bind _returnvalue (`self.GetOwner`))
  (if (`self.PickedUp`)
    (`Actor.SetActorEnableCollision` _returnvalue false)
    (else
      (`Actor.SetActorEnableCollision` _returnvalue true))))

(fn `Pickup`
  (params (Player :type "/Game/Dev/Blueprints/Entities/Players/BP_Player Object Reference"))
  (bind _returnvalue (`self.GetOwner`))
  (`Actor.K2_SetActorLocation` _returnvalue (`SceneComponent.K2_GetComponentLocation` (`/Game/Dev/Blueprints/Entities/Players/BP_Player.Attach Point` Player)) false false)
  (`Actor.K2_AttachToActor` _returnvalue Player "None" "SnapToTarget" "SnapToTarget" "SnapToTarget" true)
  (`Actor.SetActorEnableCollision` _returnvalue false)
  (set `self.PickedUp` true)
  (set `self.BackupRequiresToLookAt` (`self.RequiresToLookAt`))
  (set `self.RequiresToLookAt` false)
  (set `/Game/Dev/Blueprints/Entities/Players/BP_Player.PickedUpInteractible` self Player))

(fn `Server_OnPlayerUse`
  (params (Player :type "/Game/Dev/Blueprints/Entities/Players/BP_Player Object Reference"))
  (returns (Success :type Boolean))
  (if (`self.PickedUp`)
    (`self.Drop` Player)
    (else
      (`self.Pickup` Player)))
  (return true))