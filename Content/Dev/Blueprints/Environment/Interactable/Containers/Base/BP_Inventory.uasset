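; BP_Inventory is a size-limited item store for interactable containers, with functions to add, remove, fetch and look up items.
; AddItem uses the CanAddMore macro to reject items once the Items array reaches Size, returning whether the add succeeded.
; MoveItem transfers an item by index to another inventory, removing it from this one only if the target accepts it.
; BeginPlay and Tick are unused.
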(fn `AddItem`
  (params (Item :type "/Game/Shipping/Blueprints/Environment/Interactable/Items/Base/BP_Item Object Reference (by ref)"))
  (returns (Successful :type Boolean))
  (`self.CanAddMore`
    (:`Yes`
      (`KismetArrayLibrary.Array_Add` (`self.Items`) Item)
      (return true))
    (:`No`
      (return false))))

(fn `Get Items`
  (returns (Items :type "Array of /Game/Shipping/Blueprints/Environment/Interactable/Items/Base/BP_Item Object Reference"))
  (return (`self.Items`)))

(fn `GetItem`
  (params (ItemIndex :type Integer))
  (returns (Item :type "/Game/Shipping/Blueprints/Environment/Interactable/Items/Base/BP_Item Object Reference"))
  (return (`|GetArrayItem` (`self.Items`) ItemIndex)))

(fn `IsItemInside`
  (params (Item :type "/Game/Shipping/Blueprints/Environment/Interactable/Items/Base/BP_Item Object Reference"))
  (returns (IsInside :type Boolean))
  (for _array_element (`self.Items`)
    (if (== _array_element Item)
      (return true)))
  (return false))

(fn `MoveItem`
  (params (Inventory :type "/Game/Dev/Blueprints/Environment/Interactable/Containers/Base/BP_Inventory Object Reference (by ref)") (InvID :type Integer))
  (returns (Success :type Boolean) (RemovedItem :type "/Game/Shipping/Blueprints/Environment/Interactable/Items/Base/BP_Item Object Reference"))
  (locals (Item :type "/Game/Shipping/Blueprints/Environment/Interactable/Items/Base/BP_Item Object Reference"))
  (bind _items (`self.Items`))
  (bind _successful (`self.AddItem` Inventory (`|GetArrayItem` _items InvID)))
  (if _successful
    (bind _item (`self.GetItem` InvID))
    (bind _output_get (set `local.Item` _item))
    (`KismetArrayLibrary.Array_RemoveItem` _items _item)
    (return _successful _output_get)
    (else
      (return _successful null))))

(fn `Remove Item`
  (params (Item :type "/Game/Shipping/Blueprints/Environment/Interactable/Items/Base/BP_Item Object Reference (by ref)"))
  (bind _items (`self.Items`))
  (for _array_element _items
    (if (== _array_element Item)
      (`KismetArrayLibrary.Array_RemoveItem` _items Item)
      (break)))
  (return))