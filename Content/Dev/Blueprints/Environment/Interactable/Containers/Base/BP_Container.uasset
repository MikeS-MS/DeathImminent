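; Base container Blueprint for interactables that hand items from their own inventory to the player.
; MoveItemToTarget takes the first Player overlapping the collision component and moves the item with the given ID into that player's inventory.
; The result feeds PostActionOnOverlapAndUse, which shows an item-got widget with the item's name, or a no-item widget otherwise.
; It then calls the empty PostPostActionOnOverlapAndUse event as an extension hook.
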(event `PostActionOnOverlapAndUse`
  (params (CompletedTransfer :type Boolean) (Item :type "/Game/Shipping/Blueprints/Environment/Interactable/Items/Base/BP_Item Object Reference (by ref)"))
  (bind _returnvalue (`GameplayStatics.GetPlayerController` 0))
  (if CompletedTransfer
    (`/Engine/EditorBlueprintResources/StandardMacros.IsValid` Item
      (:`Is Valid`
        (bind _returnvalue_2 (`|CreateWidget` "/Game/Dev/Blueprints/HUD/WBP_ItemGot.WBP_ItemGot_C" _returnvalue (`KismetTextLibrary.Conv_TextToString` (`/Game/Shipping/Blueprints/Environment/Interactable/Items/Base/BP_Item.GetDisplayName` Item))))
        (`UserWidget.AddToViewport` _returnvalue_2 0))
      (:`Is Not Valid`
        (bind _returnvalue_3 (`|CreateWidget` "/Game/Dev/Blueprints/HUD/WBP_NoItem.WBP_NoItem_C" _returnvalue :!label _label))
        (`UserWidget.AddToViewport` _returnvalue_3 0)))
    (else
      (goto _label)))
  (`self.PostPostActionOnOverlapAndUse` CompletedTransfer Item))

(event `PostPostActionOnOverlapAndUse`
  (params (CompletedTransfer :type Boolean) (Item :type "/Game/Shipping/Blueprints/Environment/Interactable/Items/Base/BP_Item Object Reference")))

(fn `MoveItemToTarget`
  (params (ItemID :type Integer))
  (bind _collisioncomponent (`self.CollisionComponent`))
  (`/Engine/EditorBlueprintResources/StandardMacros.IsValid` _collisioncomponent
    (:`Is Valid`
      (bind _asplayer (cast `/Game/Shipping/Blueprints/Entities/Player` (`|GetArrayItem` (`PrimitiveComponent.GetOverlappingActors` _collisioncomponent "/Game/Shipping/Blueprints/Entities/Player.Player_C"))))
      (bind (_success _removeditem) (`/Game/Shipping/Blueprints/Environment/Interactable/Containers/Base/BP_Inventory.MoveItem` (`self.BP_Inventory`) (`/Game/Shipping/Blueprints/Entities/Player.BP_Inventory` _asplayer) ItemID))
      (`self.PostActionOnOverlapAndUse` _success _removeditem))))

(fn `UserConstructionScript`
  (`parent.UserConstructionScript`))