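; Small sliding door variant that unlocks with a matching key from the player's inventory.
; TryUnlock runs the parent logic, then scans the inventory's items for a key whose type and ID match the door's RequiredKey.
; The first match is removed from the inventory and the door unlocks.
; All other behavior is left to the parent class, as the event graph holds only disabled stubs.
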(fn `TryUnlock`
  (params (Player :type "/Game/Shipping/Blueprints/Entities/Player Object Reference (by ref)"))
  (bind _bp_inventory (`/Game/Shipping/Blueprints/Entities/Player.BP_Inventory` Player))
  (bind (_requiredkey_keytype _requiredkey_keyid) (break `/Game/Shipping/Blueprints/Environment/Interactable/Items/QuestItems/S_Key_Data` (`self.RequiredKey`)))
  (`parent.TryUnlock` Player)
  (for _array_element (`/Game/Shipping/Blueprints/Environment/Interactable/Containers/Base/BP_Inventory.Get Items` _bp_inventory)
    (bind _asbp_item_key (cast `/Game/Shipping/Blueprints/Environment/Interactable/Items/QuestItems/BP_Item_Key` _array_element))
    (if (and (== (`/Game/Shipping/Blueprints/Environment/Interactable/Items/QuestItems/BP_Item_Key.Type` _asbp_item_key) _requiredkey_keytype) (== _requiredkey_keyid (`/Game/Shipping/Blueprints/Environment/Interactable/Items/Base/BP_Item.GetItemID` _asbp_item_key)))
      (`/Game/Shipping/Blueprints/Environment/Interactable/Containers/Base/BP_Inventory.Remove Item` _bp_inventory _array_element)
      (`self.Unlock`)
      (break))))

(fn `UserConstructionScript`
  (`parent.UserConstructionScript`))